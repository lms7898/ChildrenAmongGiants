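; Box spawner blueprint that repositions a set of existing boxes when a lever is used; it spawns no new actors.
; On BeginPlay it binds its Interaction event to LeverManager1.
; Interaction teleports each entry in Boxes to a base position plus an OffsetsXYZ value, with zero rotation.
; All three axes read the same offset element, at three times the box's index.
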(event `self.ReceiveBeginPlay`
  (add `/Game/Blueprints/LeverBlueprints/LeverManager.LeverInteraction` (`self.LeverManager1`) (delegate `Interaction`)))

(event `Interaction`
  (for (_array_element _array_index) (`self.Boxes`)
    (bind _item (`KismetArrayLibrary.Array_Get` (`self.OffsetsXYZ`) (* _array_index 3)))
    (`self.K2_TeleportTo` :`self` _array_element :`DestLocation` (`KismetMathLibrary.MakeVector` (+ (`self.PositionX`) _item) (+ (`self.PositionY`) _item) (+ (`self.PositionZ`) _item)))))

(fn `UserConstructionScript`)