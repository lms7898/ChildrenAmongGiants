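; Actor component that swaps textures on the owner's skeletal mesh through a dynamic material.
; BeginPlay caches the first skeletal mesh and its slot 0 material, while a separate Init event creates and applies the dynamic instance unless one is already set.
; SetTexture writes the texture parameter once initialized, and SetTextureByName finds array entries by object name.
; Tick holds demo code that cycles the texture array every frame.
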(event `self.ReceiveBeginPlay`
  ;[1 1 1] Owner ref
  (bind _output_get (set `self.owner` (`self.GetOwner`)))
  ;[1 1 1] Get Skeletal Mesh and Material Ref
  (bind _output_get_2 (set `self.SMesh` (`KismetArrayLibrary.Array_Get` (`Actor.K2_GetComponentsByClass` _output_get "/Script/Engine.SkeletalMeshComponent"))))
  (set `self.ActorMaterial` (`PrimitiveComponent.GetMaterial` _output_get_2 0)))

(event `self.ReceiveTick`
  (params (DeltaSeconds :type "Float (single-precision)"))
  ;[1 1 1] Demo texture change ability -- delete this chunk if you are reading this
  (set `self.temp` (mod (+ (`self.temp`) 1) (`KismetArrayLibrary.Array_Length` (`self.Textures`))))
  (`self.SetTexture` (`KismetArrayLibrary.Array_Get` (`self.Textures`) (`self.temp`))))

(event `Init`
  ;[1 1 1] Check for manually set dynamic mat
  (if (not (`KismetSystemLibrary.IsValid` (`self.DynamicMaterial`)))
    ;[1 1 1] Create dynamic material instance
    (bind _returnvalue (`KismetMaterialLibrary.CreateDynamicMaterialInstance` null))
    (set `self.DynamicMaterial` _returnvalue)
    ;[1 1 1] Use Dynamic Mat on Skeletal Mesh
    (`PrimitiveComponent.SetMaterial` (`self.SMesh`) 0 (`self.DynamicMaterial`)))
  ;[1 1 1] Initialized flag
  (set `self.Initialized` true))

(fn `GetTextureByName`
  (params (name :type String))
  (returns (Texture :type "Texture Object Reference"))
  (for _array_element (`self.Textures`)
    (if (`KismetStringLibrary.EqualEqual_StrStr` (`KismetSystemLibrary.GetObjectName` _array_element) name)
      (return _array_element)))
  (return _array_element))

(fn `SetTexture`
  (params (Tex :type "Texture Object Reference"))
  (if (`self.Initialized`)
    (`MaterialInstanceDynamic.SetTextureParameterValue` (`self.DynamicMaterial`) "TextureParam" Tex)
    (return)
    (else
      (return))))

(fn `SetTextureByName`
  (params (Name :type String))
  (bind _texture (`self.GetTextureByName` Name))
  (`self.SetTexture` _texture))