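; CameraZoomChange is a trigger actor that changes the third-person camera zoom when the character overlaps it.
; On overlap it records the camera boom's current arm length, the difference to its target length and the zoom direction.
; Tick then linearly interpolates the player 0 character's arm length over the zoom duration, snapping to the target and stopping once the time elapses.
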(event `self.ReceiveActorBeginOverlap`
  (params (OtherActor :type "Actor Object Reference"))
  ;[1 1 1] Initial Values
  (bind _asthird_person_character (cast `/Game/Blueprints/Player/ThirdPersonCharacter` OtherActor))
  (set `self.TimePassed` 0.0)
  (bind _output_get (set `self.CameraZoomStart` (`SpringArmComponent.TargetArmLength` (`/Game/Blueprints/Player/ThirdPersonCharacter.CameraBoom` _asthird_person_character))))
  (bind _output_get_2 (set `self.CameraZoomDifference` (- (`self.CameraZoomEnd`) _output_get)))
  (if (== _output_get_2 0.0)
    (set `self.ZoomEqual` true)
    (else
      (set `self.ZoomGrowing` (> _output_get_2 0.0))
      (set `self.ZoomEqual` false))))

(event `self.ReceiveTick`
  (params (DeltaSeconds :type "Float (single-precision)"))
  (bind _camerazoomend (`self.CameraZoomEnd`))
  (if (not (`self.ZoomEqual`))
    (bind _asthird_person_character (cast `/Game/Blueprints/Player/ThirdPersonCharacter` (`GameplayStatics.GetPlayerCharacter` 0)))
    (if (`self.ZoomGrowing`)
      (bind _cameraboom (`/Game/Blueprints/Player/ThirdPersonCharacter.CameraBoom` _asthird_person_character))
      (bind _targetarmlength (`SpringArmComponent.TargetArmLength` _cameraboom))
      ;[1 1 1] Zoom
      (if (< _targetarmlength _camerazoomend)
        (bind _output_get (set `self.TimePassed` (+ DeltaSeconds (`self.TimePassed`)) :!label _label))
        (if (< _output_get (`self.ZoomDuration`))
          (set `SpringArmComponent.TargetArmLength` (+ (* (`self.CameraZoomDifference`) (/ (`self.TimePassed`) (`self.ZoomDuration`))) (`self.CameraZoomStart`)) _cameraboom)
          (else
            (set `SpringArmComponent.TargetArmLength` (`self.CameraZoomEnd`) _cameraboom)
            (set `self.ZoomEqual` true))))
      (elif (> _targetarmlength _camerazoomend)
        (goto _label)))))

(fn `UserConstructionScript`)