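; Level-specific lighthouse Blueprint that tracks whether the player character, Dusk, counts as being in the lighthouse beam.
; Each tick it line traces from its owner's location to Dusk and sets PlayerInBeam when Dusk is the hit actor.
; The trace queries only Pawn objects and checks no beam direction or angle.
; A graph for raising or lowering Dusk's remaining light ability is present but unconnected, so it never runs.
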(event `self.ReceiveBeginPlay`
  (set `self.Dusk` (cast `/Game/Blueprints/Player/ThirdPersonCharacter` (`GameplayStatics.GetPlayerCharacter` 0) :!pure true)))

(event `self.ReceiveTick`
  (params (DeltaSeconds :type "Float (single-precision)"))
  ;[1 1 1] Player is in the lighthouse beam or not
  (bind _outhit (`KismetSystemLibrary.LineTraceSingleForObjects` :`Start` (`Actor.K2_GetActorLocation` (`self.GetOwner`)) :`End` (`Actor.K2_GetActorLocation` (`self.Dusk`)) :`ObjectTypes` (`|MakeArray` "ObjectTypeQuery3" :!type "EObjectTypeQuery Enum") :`bIgnoreSelf` false))
  (set `self.PlayerInBeam` (== (`self.Dusk`) (`.HitActor` (`GameplayStatics.BreakHitResult` _outhit)))))