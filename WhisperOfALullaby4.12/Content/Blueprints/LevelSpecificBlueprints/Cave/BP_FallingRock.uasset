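; BP_FallingRock is a cave level hazard: a physics rock that repeatedly drops and damages the player character.
; It stores the rock's starting location on BeginPlay, then uses a Delay on Tick as a repeating timer to move it back there and zero its velocity.
; Each hit on a ThirdPersonCharacter subtracts one directly from that character's CurrentHealth.
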(event `self.ReceiveBeginPlay`
  (set `self.Position` (`SceneComponent.K2_GetComponentLocation` (`self.Rock`))))

(event `self.ReceiveTick`
  (params (DeltaSeconds :type "Float (single-precision)"))
  (bind _rock (`self.Rock`))
  (`KismetSystemLibrary.Delay` (`self.DelayTime`))
  (`SceneComponent.K2_SetWorldLocation` _rock (`self.Position`) false false)
  (`PrimitiveComponent.SetAllPhysicsLinearVelocity` _rock (0.0 0.0 0.0) false))

(event `self.Rock.OnComponentHit`
  (params (HitComponent :type "PrimitiveComponent Object Reference") (OtherActor :type "Actor Object Reference") (OtherComp :type "PrimitiveComponent Object Reference") (NormalImpulse :type "Vector Structure") (Hit :type "HitResult Structure (by ref)"))
  (bind _asthird_person_character (cast `/Game/Blueprints/Player/ThirdPersonCharacter` OtherActor))
  (set `/Game/Blueprints/Player/ThirdPersonCharacter.CurrentHealth` (- (`/Game/Blueprints/Player/ThirdPersonCharacter.CurrentHealth` _asthird_person_character) 1) _asthird_person_character))

(fn `UserConstructionScript`)