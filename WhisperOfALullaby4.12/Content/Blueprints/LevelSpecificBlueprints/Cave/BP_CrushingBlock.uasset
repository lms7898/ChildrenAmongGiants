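; BP_CrushingBlock is a cave-level hazard block that damages the third-person character on overlap.
; On BeginPlay it stores Block1's starting location, then wakes the block's rigid body after a short delay so physics can act on it.
; Any actor overlap that casts to ThirdPersonCharacter subtracts one from CurrentHealth.
; The saved StartPos is not read in these graphs, and nothing here resets the block.
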(event `self.ReceiveBeginPlay`
  (`|ExecutionSequence`
    (:`then_0`
      (set `self.Start_Pos` (`SceneComponent.K2_GetComponentLocation` (`self.Block1`))))
    (:`then_1`
      (`KismetSystemLibrary.Delay` 2.0)
      (`PrimitiveComponent.WakeRigidBody` (`self.Block1`) "None"))))

(event `self.ReceiveActorBeginOverlap`
  (params (OtherActor :type "Actor Object Reference"))
  (bind _asthird_person_character (cast `/Game/Blueprints/Player/ThirdPersonCharacter` OtherActor))
  (set `/Game/Blueprints/Player/ThirdPersonCharacter.CurrentHealth` (- (`/Game/Blueprints/Player/ThirdPersonCharacter.CurrentHealth` _asthird_person_character) 1) _asthird_person_character))

(fn `UserConstructionScript`)