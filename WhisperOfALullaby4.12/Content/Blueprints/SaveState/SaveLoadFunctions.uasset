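; Save/load function set that moves WoaL game progress between the Game Instance and save slots: level, music box pieces, ability unlocks, Level 1 flags and checkpoint.
; SaveGame writes the full save plus a separate meta save holding level, checkpoint index and timestamp, readable alone through LoadMetaData.
; Saving and loading set the active slot pair.
; ValuesToLoadFull writes the saved Arty unlock into EllianaAbilityUnlocked, leaving ArtyAbilityUnlocked unrestored.
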(fn SaveGame
  (params (SaveSlot :type String) (MetaSlot :type String))
  (LocalVariables|SetSaveGameSlot SaveSlot)
  (LocalVariables|SetMetaDataSlot MetaSlot)
  ;[1 1 1] Set Game Instance Ref
  (bind _aswoa_lgame_instance (Utilities|Casting|CastToWoaLGameInstance (Game|GetGameInstance)))
  (bind _output_get (LocalVariables|SetGameInstanceRef _aswoa_lgame_instance))
  ;[1 1 1] Designate Auto Save Slots
  (Variables|/Game/GameInstances/WoaLGameInstance.WoaLGameInstance_C|SetActiveMetaSlot _output_get (LocalVariables|GetMetaDataSlot))
  (Variables|/Game/GameInstances/WoaLGameInstance.WoaLGameInstance_C|SetActiveSaveSlot _output_get (LocalVariables|GetSaveGameSlot))
  ;[1 1 1] Save Game
  (bind _returnvalue (SaveGame|CreateSaveGameObject "/Game/Blueprints/SaveState/WoaLSaveGame.WoaLSaveGame_C"))
  (bind _aswoa_lsave_game (Utilities|Casting|CastToWoaLSaveGame _returnvalue))
  (bind _output_get_2 (LocalVariables|SetWoaLSaveGameRef _aswoa_lsave_game))
  (CallFunction|ValuestoSaveFull _output_get_2 (LocalVariables|GetGameInstanceRef))
  (SaveGame|SaveGametoSlot _output_get_2 (LocalVariables|GetSaveGameSlot))
  ;[1 1 1] Save Meta Data
  (bind _returnvalue_2 (SaveGame|CreateSaveGameObject "/Game/Blueprints/SaveState/WoaLSaveGameMeta.WoaLSaveGameMeta_C"))
  (bind _aswoa_lsave_game_meta (Utilities|Casting|CastToWoaLSaveGameMeta _returnvalue_2))
  (bind _output_get_3 (LocalVariables|SetWoaLMetaDataRef _aswoa_lsave_game_meta))
  (CallFunction|SaveMetaData _output_get_3 (LocalVariables|GetGameInstanceRef))
  (SaveGame|SaveGametoSlot _output_get_3 (LocalVariables|GetMetaDataSlot)))

(fn LoadGame
  (params (SaveSlot :type String))
  (LocalVariables|SetSaveGameSlot SaveSlot)
  ;[1 1 1] Set Game Instance Ref
  (bind _aswoa_lgame_instance (Utilities|Casting|CastToWoaLGameInstance (Game|GetGameInstance)))
  (LocalVariables|SetGameInstanceRef _aswoa_lgame_instance)
  ;[1 1 1] Check if the Save Game Exists
  (bind _returnvalue (SaveGame|DoesSaveGameExist (LocalVariables|GetSaveGameSlot)))
  (if _returnvalue
    ;[1 1 1] Load Game
    (bind _returnvalue_2 (SaveGame|LoadGamefromSlot (LocalVariables|GetSaveGameSlot)))
    (bind _output_get (LocalVariables|SetBP_SaveGame _returnvalue_2))
    (bind _aswoa_lsave_game (Utilities|Casting|CastToWoaLSaveGame _output_get))
    (LocalVariables|SetWoaLSaveGameRef _aswoa_lsave_game)
    ;;[1 1 1] Update Game Instance
    (CallFunction|ValuestoLoadFull (LocalVariables|GetGameInstanceRef) (LocalVariables|GetWoaLSaveGameRef))
    ;[1 1 1] Designate Auto Save Slots
    (switch string (LocalVariables|GetSaveGameSlot)
      (:WoaLSave1
        (Variables|/Game/GameInstances/WoaLGameInstance.WoaLGameInstance_C|SetActiveMetaSlot (LocalVariables|GetGameInstanceRef) "WoaLMeta1"))
      (:WoaLSave2
        (Variables|/Game/GameInstances/WoaLGameInstance.WoaLGameInstance_C|SetActiveMetaSlot (LocalVariables|GetGameInstanceRef) "WoaLMeta2"))
      (:WoaLSave3
        (Variables|/Game/GameInstances/WoaLGameInstance.WoaLGameInstance_C|SetActiveMetaSlot (LocalVariables|GetGameInstanceRef) "WoaLMeta3"))
      (:WoaLSave4
        (Variables|/Game/GameInstances/WoaLGameInstance.WoaLGameInstance_C|SetActiveMetaSlot (LocalVariables|GetGameInstanceRef) "WoaLMeta4")))
    (Variables|/Game/GameInstances/WoaLGameInstance.WoaLGameInstance_C|SetActiveSaveSlot (LocalVariables|GetGameInstanceRef) (LocalVariables|GetSaveGameSlot))))

(fn ValuestoSaveFull
  (params (SaveGameRef :type Woa%20L%20Save%20Game%20Object%20Reference) (GameInstRef :type Woa%20L%20Game%20Instance%20Object%20Reference))
  ;[1 1 1] Current Level
  (Variables|/Game/Blueprints/SaveState/WoaLSaveGame.WoaLSaveGame_C|SetS_CurrentLevel SaveGameRef (Variables|/Game/GameInstances/WoaLGameInstance.WoaLGameInstance_C|GetCurrentLevel GameInstRef))
  ;[1 1 1] Music Box Pieces
  (Variables|/Game/Blueprints/SaveState/WoaLSaveGame.WoaLSaveGame_C|SetS_MBElli1 SaveGameRef (Variables|/Game/GameInstances/WoaLGameInstance.WoaLGameInstance_C|GetMBElli1 GameInstRef))
  (Variables|/Game/Blueprints/SaveState/WoaLSaveGame.WoaLSaveGame_C|SetS_MBElli2 SaveGameRef (Variables|/Game/GameInstances/WoaLGameInstance.WoaLGameInstance_C|GetMBElli2 GameInstRef))
  (Variables|/Game/Blueprints/SaveState/WoaLSaveGame.WoaLSaveGame_C|SetS_MBElli3 SaveGameRef (Variables|/Game/GameInstances/WoaLGameInstance.WoaLGameInstance_C|GetMBElli3 GameInstRef))
  (Variables|/Game/Blueprints/SaveState/WoaLSaveGame.WoaLSaveGame_C|SetS_MBElli4 SaveGameRef (Variables|/Game/GameInstances/WoaLGameInstance.WoaLGameInstance_C|GetMBElli4 GameInstRef))
  (Variables|/Game/Blueprints/SaveState/WoaLSaveGame.WoaLSaveGame_C|SetS_MBElli5 SaveGameRef (Variables|/Game/GameInstances/WoaLGameInstance.WoaLGameInstance_C|GetMBElli5 GameInstRef))
  (Variables|/Game/Blueprints/SaveState/WoaLSaveGame.WoaLSaveGame_C|SetS_MBHelios1 SaveGameRef (Variables|/Game/GameInstances/WoaLGameInstance.WoaLGameInstance_C|GetMBHelios1 GameInstRef))
  (Variables|/Game/Blueprints/SaveState/WoaLSaveGame.WoaLSaveGame_C|SetS_MBHelios2 SaveGameRef (Variables|/Game/GameInstances/WoaLGameInstance.WoaLGameInstance_C|GetMBHelios2 GameInstRef))
  (Variables|/Game/Blueprints/SaveState/WoaLSaveGame.WoaLSaveGame_C|SetS_MBHelios3 SaveGameRef (Variables|/Game/GameInstances/WoaLGameInstance.WoaLGameInstance_C|GetMBHelios3 GameInstRef))
  (Variables|/Game/Blueprints/SaveState/WoaLSaveGame.WoaLSaveGame_C|SetS_MBHelios4 SaveGameRef (Variables|/Game/GameInstances/WoaLGameInstance.WoaLGameInstance_C|GetMBHelios4 GameInstRef))
  (Variables|/Game/Blueprints/SaveState/WoaLSaveGame.WoaLSaveGame_C|SetS_MBHelios5 SaveGameRef (Variables|/Game/GameInstances/WoaLGameInstance.WoaLGameInstance_C|GetMBHelios5 GameInstRef))
  ;[1 1 1] Ability Unlocks
  (Variables|/Game/Blueprints/SaveState/WoaLSaveGame.WoaLSaveGame_C|SetS_EllianaAbilityUnlocked SaveGameRef (Variables|/Game/GameInstances/WoaLGameInstance.WoaLGameInstance_C|GetEllianaAbilityUnlocked GameInstRef))
  (Variables|/Game/Blueprints/SaveState/WoaLSaveGame.WoaLSaveGame_C|SetS_HeliosAbilityUnlocked SaveGameRef (Variables|/Game/GameInstances/WoaLGameInstance.WoaLGameInstance_C|GetHeliosAbilityUnlocked GameInstRef))
  (Variables|/Game/Blueprints/SaveState/WoaLSaveGame.WoaLSaveGame_C|SetS_StarlightAbilityUnlocked SaveGameRef (Variables|/Game/GameInstances/WoaLGameInstance.WoaLGameInstance_C|GetStarlightAbilityUnlocked GameInstRef))
  (Variables|/Game/Blueprints/SaveState/WoaLSaveGame.WoaLSaveGame_C|SetS_ArtyAbilityUnlocked SaveGameRef (Variables|/Game/GameInstances/WoaLGameInstance.WoaLGameInstance_C|GetArtyAbilityUnlocked GameInstRef))
  (Variables|/Game/Blueprints/SaveState/WoaLSaveGame.WoaLSaveGame_C|SetS_SerenAbilityUnlocked SaveGameRef (Variables|/Game/GameInstances/WoaLGameInstance.WoaLGameInstance_C|GetSerenAbilityUnlocked GameInstRef))
  (Variables|/Game/Blueprints/SaveState/WoaLSaveGame.WoaLSaveGame_C|SetS_AtlasAbilityUnlocked SaveGameRef (Variables|/Game/GameInstances/WoaLGameInstance.WoaLGameInstance_C|GetAtlasAbilityUnlocked GameInstRef))
  (Variables|/Game/Blueprints/SaveState/WoaLSaveGame.WoaLSaveGame_C|SetS_LunaAbilityUnlocked SaveGameRef (Variables|/Game/GameInstances/WoaLGameInstance.WoaLGameInstance_C|GetLunaAbilityUnlocked GameInstRef))
  ;[1 1 1] Level 1 Booleans
  (Variables|/Game/Blueprints/SaveState/WoaLSaveGame.WoaLSaveGame_C|SetS_D_HouseOnHill SaveGameRef (Variables|/Game/GameInstances/WoaLGameInstance.WoaLGameInstance_C|GetD_HouseOnHill GameInstRef))
  (Variables|/Game/Blueprints/SaveState/WoaLSaveGame.WoaLSaveGame_C|SetS_D_JumpingFence SaveGameRef (Variables|/Game/GameInstances/WoaLGameInstance.WoaLGameInstance_C|GetD_JumpingFence GameInstRef))
  (Variables|/Game/Blueprints/SaveState/WoaLSaveGame.WoaLSaveGame_C|SetS_D_ClearingRubble SaveGameRef (Variables|/Game/GameInstances/WoaLGameInstance.WoaLGameInstance_C|GetD_ClearingRubble GameInstRef))
  (Variables|/Game/Blueprints/SaveState/WoaLSaveGame.WoaLSaveGame_C|SetS_D_Clocktower SaveGameRef (Variables|/Game/GameInstances/WoaLGameInstance.WoaLGameInstance_C|GetD_Clocktower GameInstRef))
  (Variables|/Game/Blueprints/SaveState/WoaLSaveGame.WoaLSaveGame_C|SetS_D_EnteringMarket SaveGameRef (Variables|/Game/GameInstances/WoaLGameInstance.WoaLGameInstance_C|GetD_EnteringMarket GameInstRef))
  (Variables|/Game/Blueprints/SaveState/WoaLSaveGame.WoaLSaveGame_C|SetS_D_MarketGateDestroyed SaveGameRef (Variables|/Game/GameInstances/WoaLGameInstance.WoaLGameInstance_C|GetD_MarketGateDestroyed GameInstRef))
  (Variables|/Game/Blueprints/SaveState/WoaLSaveGame.WoaLSaveGame_C|SetS_D_EnteringNeighborhood SaveGameRef (Variables|/Game/GameInstances/WoaLGameInstance.WoaLGameInstance_C|GetD_EnteringNeighborhood GameInstRef))
  (Variables|/Game/Blueprints/SaveState/WoaLSaveGame.WoaLSaveGame_C|SetS_D_ElliHouse1 SaveGameRef (Variables|/Game/GameInstances/WoaLGameInstance.WoaLGameInstance_C|GetD_ElliHouse1 GameInstRef))
  (Variables|/Game/Blueprints/SaveState/WoaLSaveGame.WoaLSaveGame_C|SetS_D_ElliHouse2 SaveGameRef (Variables|/Game/GameInstances/WoaLGameInstance.WoaLGameInstance_C|GetD_ElliHouse2 GameInstRef))
  (Variables|/Game/Blueprints/SaveState/WoaLSaveGame.WoaLSaveGame_C|SetS_D_ElliHouse3 SaveGameRef (Variables|/Game/GameInstances/WoaLGameInstance.WoaLGameInstance_C|GetD_ElliHouse3 GameInstRef))
  (Variables|/Game/Blueprints/SaveState/WoaLSaveGame.WoaLSaveGame_C|SetS_D_DontWorryAboutMonsters SaveGameRef (Variables|/Game/GameInstances/WoaLGameInstance.WoaLGameInstance_C|GetD_DontWorryAboutMonsters GameInstRef))
  (Variables|/Game/Blueprints/SaveState/WoaLSaveGame.WoaLSaveGame_C|SetS_D_WorryAboutMonsters SaveGameRef (Variables|/Game/GameInstances/WoaLGameInstance.WoaLGameInstance_C|GetD_WorryAboutMonsters GameInstRef))
  (Variables|/Game/Blueprints/SaveState/WoaLSaveGame.WoaLSaveGame_C|SetS_MarketGateDestroyed SaveGameRef (Variables|/Game/GameInstances/WoaLGameInstance.WoaLGameInstance_C|GetMarketGateDestroyed GameInstRef))
  (Variables|/Game/Blueprints/SaveState/WoaLSaveGame.WoaLSaveGame_C|SetS_MarketGateKey1 SaveGameRef (Variables|/Game/GameInstances/WoaLGameInstance.WoaLGameInstance_C|GetMarketGateKey1 GameInstRef))
  (Variables|/Game/Blueprints/SaveState/WoaLSaveGame.WoaLSaveGame_C|SetS_MarketGateKey2 SaveGameRef (Variables|/Game/GameInstances/WoaLGameInstance.WoaLGameInstance_C|GetMarketGateKey2 GameInstRef))
  ;[1 1 1] Checkpoints
  (Variables|/Game/Blueprints/SaveState/WoaLSaveGame.WoaLSaveGame_C|SetS_CheckpointTransform SaveGameRef (Variables|/Game/GameInstances/WoaLGameInstance.WoaLGameInstance_C|GetCheckpointTransform GameInstRef))
  (Variables|/Game/Blueprints/SaveState/WoaLSaveGame.WoaLSaveGame_C|SetS_CheckpointIndex SaveGameRef (Variables|/Game/GameInstances/WoaLGameInstance.WoaLGameInstance_C|GetCheckpointIndex GameInstRef))
  (return))

(fn ValuestoLoadFull
  (params (GameInstRef :type Woa%20L%20Game%20Instance%20Object%20Reference) (SaveGameRef :type Woa%20L%20Save%20Game%20Object%20Reference))
  ;[1 1 1] Current Level
  (Variables|/Game/GameInstances/WoaLGameInstance.WoaLGameInstance_C|SetCurrentLevel GameInstRef (Variables|/Game/Blueprints/SaveState/WoaLSaveGame.WoaLSaveGame_C|GetS_CurrentLevel SaveGameRef))
  ;[1 1 1] Music Box Pieces
  (Variables|/Game/GameInstances/WoaLGameInstance.WoaLGameInstance_C|SetMBElli1 GameInstRef (Variables|/Game/Blueprints/SaveState/WoaLSaveGame.WoaLSaveGame_C|GetS_MBElli1 SaveGameRef))
  (Variables|/Game/GameInstances/WoaLGameInstance.WoaLGameInstance_C|SetMBElli2 GameInstRef (Variables|/Game/Blueprints/SaveState/WoaLSaveGame.WoaLSaveGame_C|GetS_MBElli2 SaveGameRef))
  (Variables|/Game/GameInstances/WoaLGameInstance.WoaLGameInstance_C|SetMBElli3 GameInstRef (Variables|/Game/Blueprints/SaveState/WoaLSaveGame.WoaLSaveGame_C|GetS_MBElli3 SaveGameRef))
  (Variables|/Game/GameInstances/WoaLGameInstance.WoaLGameInstance_C|SetMBElli4 GameInstRef (Variables|/Game/Blueprints/SaveState/WoaLSaveGame.WoaLSaveGame_C|GetS_MBElli4 SaveGameRef))
  (Variables|/Game/GameInstances/WoaLGameInstance.WoaLGameInstance_C|SetMBElli5 GameInstRef (Variables|/Game/Blueprints/SaveState/WoaLSaveGame.WoaLSaveGame_C|GetS_MBElli5 SaveGameRef))
  (Variables|/Game/GameInstances/WoaLGameInstance.WoaLGameInstance_C|SetMBHelios1 GameInstRef (Variables|/Game/Blueprints/SaveState/WoaLSaveGame.WoaLSaveGame_C|GetS_MBHelios1 SaveGameRef))
  (Variables|/Game/GameInstances/WoaLGameInstance.WoaLGameInstance_C|SetMBHelios2 GameInstRef (Variables|/Game/Blueprints/SaveState/WoaLSaveGame.WoaLSaveGame_C|GetS_MBHelios2 SaveGameRef))
  (Variables|/Game/GameInstances/WoaLGameInstance.WoaLGameInstance_C|SetMBHelios3 GameInstRef (Variables|/Game/Blueprints/SaveState/WoaLSaveGame.WoaLSaveGame_C|GetS_MBHelios3 SaveGameRef))
  (Variables|/Game/GameInstances/WoaLGameInstance.WoaLGameInstance_C|SetMBHelios4 GameInstRef (Variables|/Game/Blueprints/SaveState/WoaLSaveGame.WoaLSaveGame_C|GetS_MBHelios4 SaveGameRef))
  (Variables|/Game/GameInstances/WoaLGameInstance.WoaLGameInstance_C|SetMBHelios5 GameInstRef (Variables|/Game/Blueprints/SaveState/WoaLSaveGame.WoaLSaveGame_C|GetS_MBHelios5 SaveGameRef))
  ;[1 1 1] Ability Unlocks
  (Variables|/Game/GameInstances/WoaLGameInstance.WoaLGameInstance_C|SetEllianaAbilityUnlocked GameInstRef (Variables|/Game/Blueprints/SaveState/WoaLSaveGame.WoaLSaveGame_C|GetS_EllianaAbilityUnlocked SaveGameRef))
  (Variables|/Game/GameInstances/WoaLGameInstance.WoaLGameInstance_C|SetHeliosAbilityUnlocked GameInstRef (Variables|/Game/Blueprints/SaveState/WoaLSaveGame.WoaLSaveGame_C|GetS_HeliosAbilityUnlocked SaveGameRef))
  (Variables|/Game/GameInstances/WoaLGameInstance.WoaLGameInstance_C|SetStarlightAbilityUnlocked GameInstRef (Variables|/Game/Blueprints/SaveState/WoaLSaveGame.WoaLSaveGame_C|GetS_StarlightAbilityUnlocked SaveGameRef))
  (Variables|/Game/GameInstances/WoaLGameInstance.WoaLGameInstance_C|SetEllianaAbilityUnlocked GameInstRef (Variables|/Game/Blueprints/SaveState/WoaLSaveGame.WoaLSaveGame_C|GetS_ArtyAbilityUnlocked SaveGameRef))
  (Variables|/Game/GameInstances/WoaLGameInstance.WoaLGameInstance_C|SetSerenAbilityUnlocked GameInstRef (Variables|/Game/Blueprints/SaveState/WoaLSaveGame.WoaLSaveGame_C|GetS_SerenAbilityUnlocked SaveGameRef))
  (Variables|/Game/GameInstances/WoaLGameInstance.WoaLGameInstance_C|SetAtlasAbilityUnlocked GameInstRef (Variables|/Game/Blueprints/SaveState/WoaLSaveGame.WoaLSaveGame_C|GetS_AtlasAbilityUnlocked SaveGameRef))
  (Variables|/Game/GameInstances/WoaLGameInstance.WoaLGameInstance_C|SetLunaAbilityUnlocked GameInstRef (Variables|/Game/Blueprints/SaveState/WoaLSaveGame.WoaLSaveGame_C|GetS_LunaAbilityUnlocked SaveGameRef))
  ;[1 1 1] Level 1 Booleans
  (Variables|/Game/GameInstances/WoaLGameInstance.WoaLGameInstance_C|SetD_HouseOnHill GameInstRef (Variables|/Game/Blueprints/SaveState/WoaLSaveGame.WoaLSaveGame_C|GetS_D_HouseOnHill SaveGameRef))
  (Variables|/Game/GameInstances/WoaLGameInstance.WoaLGameInstance_C|SetD_JumpingFence GameInstRef (Variables|/Game/Blueprints/SaveState/WoaLSaveGame.WoaLSaveGame_C|GetS_D_JumpingFence SaveGameRef))
  (Variables|/Game/GameInstances/WoaLGameInstance.WoaLGameInstance_C|SetD_ClearingRubble GameInstRef (Variables|/Game/Blueprints/SaveState/WoaLSaveGame.WoaLSaveGame_C|GetS_D_ClearingRubble SaveGameRef))
  (Variables|/Game/GameInstances/WoaLGameInstance.WoaLGameInstance_C|SetD_Clocktower GameInstRef (Variables|/Game/Blueprints/SaveState/WoaLSaveGame.WoaLSaveGame_C|GetS_D_Clocktower SaveGameRef))
  (Variables|/Game/GameInstances/WoaLGameInstance.WoaLGameInstance_C|SetD_EnteringMarket GameInstRef (Variables|/Game/Blueprints/SaveState/WoaLSaveGame.WoaLSaveGame_C|GetS_D_EnteringMarket SaveGameRef))
  (Variables|/Game/GameInstances/WoaLGameInstance.WoaLGameInstance_C|SetD_MarketGateDestroyed GameInstRef (Variables|/Game/Blueprints/SaveState/WoaLSaveGame.WoaLSaveGame_C|GetS_D_MarketGateDestroyed SaveGameRef))
  (Variables|/Game/GameInstances/WoaLGameInstance.WoaLGameInstance_C|SetD_EnteringNeighborhood GameInstRef (Variables|/Game/Blueprints/SaveState/WoaLSaveGame.WoaLSaveGame_C|GetS_D_EnteringNeighborhood SaveGameRef))
  (Variables|/Game/GameInstances/WoaLGameInstance.WoaLGameInstance_C|SetD_ElliHouse1 GameInstRef (Variables|/Game/Blueprints/SaveState/WoaLSaveGame.WoaLSaveGame_C|GetS_D_ElliHouse1 SaveGameRef))
  (Variables|/Game/GameInstances/WoaLGameInstance.WoaLGameInstance_C|SetD_ElliHouse2 GameInstRef (Variables|/Game/Blueprints/SaveState/WoaLSaveGame.WoaLSaveGame_C|GetS_D_ElliHouse2 SaveGameRef))
  (Variables|/Game/GameInstances/WoaLGameInstance.WoaLGameInstance_C|SetD_ElliHouse3 GameInstRef (Variables|/Game/Blueprints/SaveState/WoaLSaveGame.WoaLSaveGame_C|GetS_D_ElliHouse3 SaveGameRef))
  (Variables|/Game/GameInstances/WoaLGameInstance.WoaLGameInstance_C|SetD_DontWorryAboutMonsters GameInstRef (Variables|/Game/Blueprints/SaveState/WoaLSaveGame.WoaLSaveGame_C|GetS_D_DontWorryAboutMonsters SaveGameRef))
  (Variables|/Game/GameInstances/WoaLGameInstance.WoaLGameInstance_C|SetD_WorryAboutMonsters GameInstRef (Variables|/Game/Blueprints/SaveState/WoaLSaveGame.WoaLSaveGame_C|GetS_D_WorryAboutMonsters SaveGameRef))
  (Variables|/Game/GameInstances/WoaLGameInstance.WoaLGameInstance_C|SetMarketGateDestroyed GameInstRef (Variables|/Game/Blueprints/SaveState/WoaLSaveGame.WoaLSaveGame_C|GetS_MarketGateDestroyed SaveGameRef))
  (Variables|/Game/GameInstances/WoaLGameInstance.WoaLGameInstance_C|SetMarketGateKey1 GameInstRef (Variables|/Game/Blueprints/SaveState/WoaLSaveGame.WoaLSaveGame_C|GetS_MarketGateKey1 SaveGameRef))
  (Variables|/Game/GameInstances/WoaLGameInstance.WoaLGameInstance_C|SetMarketGateKey2 GameInstRef (Variables|/Game/Blueprints/SaveState/WoaLSaveGame.WoaLSaveGame_C|GetS_MarketGateKey2 SaveGameRef))
  ;[1 1 1] Checkpoints
  (Variables|/Game/GameInstances/WoaLGameInstance.WoaLGameInstance_C|SetCheckpointTransform GameInstRef (Variables|/Game/Blueprints/SaveState/WoaLSaveGame.WoaLSaveGame_C|GetS_CheckpointTransform SaveGameRef))
  (Variables|/Game/GameInstances/WoaLGameInstance.WoaLGameInstance_C|SetCheckpointIndex GameInstRef (Variables|/Game/Blueprints/SaveState/WoaLSaveGame.WoaLSaveGame_C|GetS_CheckpointIndex SaveGameRef))
  (return))

(fn SaveMetaData
  (params (MetaDataRef :type Woa%20L%20Save%20Game%20Meta%20Object%20Reference) (GameInstRef :type Woa%20L%20Game%20Instance%20Object%20Reference))
  (Variables|/Game/Blueprints/SaveState/WoaLSaveGameMeta.WoaLSaveGameMeta_C|SetMeta_CurrentLevel MetaDataRef (Variables|/Game/GameInstances/WoaLGameInstance.WoaLGameInstance_C|GetCurrentLevel GameInstRef))
  (Variables|/Game/Blueprints/SaveState/WoaLSaveGameMeta.WoaLSaveGameMeta_C|SetMeta_CheckpointIndex MetaDataRef (Variables|/Game/GameInstances/WoaLGameInstance.WoaLGameInstance_C|GetCheckpointIndex GameInstRef))
  (Variables|/Game/Blueprints/SaveState/WoaLSaveGameMeta.WoaLSaveGameMeta_C|SetMeta_DateAndTimeOfSave MetaDataRef (Math|DateTime|Now))
  (return))

(fn LoadMetaData
  (params (MetaData :type String))
  (bind _output_get (LocalVariables|SetMetaDataSlot MetaData))
  (bind _returnvalue (SaveGame|DoesSaveGameExist _output_get))
  (if _returnvalue
    ;[1 1 1] Load Game
    (bind _returnvalue_2 (SaveGame|LoadGamefromSlot (LocalVariables|GetMetaDataSlot)))
    (bind _aswoa_lsave_game_meta (Utilities|Casting|CastToWoaLSaveGameMeta _returnvalue_2)
      (:then
        (return true _aswoa_lsave_game_meta))
      (:CastFailed
        (return false 0)))
    (else
      (return false 0))))