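; Utility manager that tracks shovel pickups and use, and handles cleanup of a shovel dialogue owner.
; ShovelGet and ShovelUsed set or clear the indexed flag in ShovelFound, with a pickup also spawning an Elliana_BeachFollower near the player as HelperElli.
; DestroyShovel calls a custom event that waits briefly before destroying ShovelDialogueOwner and HelperElli, letting a function trigger latent cleanup.
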(event `ShovelGet`
  (params (index :type Integer))
  ;[1 1 1] Register Shovel Found
  (`KismetArrayLibrary.Array_Set` (`self.ShovelFound`) index true true)
  (bind _returnvalue (`|SpawnActorFromClass` "/Game/Blueprints/NPCs/Elliana_BeachFollower.Elliana_BeachFollower_C" (`KismetMathLibrary.Conv_VectorToTransform` (- (`self.K2_GetActorLocation` (`GameplayStatics.GetPlayerCharacter` 0)) 10)) "Undefined" "OverrideRootScale"))
  (set `self.HelperElli` _returnvalue))

(event `ShovelUsed`
  (params (index :type Integer))
  ;[1 1 1] Register Shovel Used
  (`KismetArrayLibrary.Array_Set` (`self.ShovelFound`) index false true))

(event `DelayedDestroyShovel`
  (`KismetSystemLibrary.Delay` 0.05)
  (`self.K2_DestroyActor` (`self.ShovelDialogueOwner`))
  (`self.K2_DestroyActor` (`self.HelperElli`)))

(fn `DestroyShovel`
  (`self.DelayedDestroyShovel`))

(fn `UserConstructionScript`)