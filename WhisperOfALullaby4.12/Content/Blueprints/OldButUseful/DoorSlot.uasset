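; DoorSlot is a key slot actor that reacts when a matching colored key overlaps it.
; On overlap, it checks the other actor for a tag equal to its KeyTag, then brightens its Light.
; A switch on KeyTag calls the matching Cyan, Orange, Green or Purple function on the referenced Opener.
; The slot has no reset or end-overlap logic.
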(event `self.ReceiveActorBeginOverlap`
  (params (OtherActor :type "Actor Object Reference"))
  (bind _opener (`self.opener`))
  (bind _keytag (`self.KeyTag`))
  (if (`self.ActorHasTag` OtherActor (`KismetStringLibrary.Conv_StringToName` _keytag))
    (`LightComponent.SetIntensity` (`self.Light`) 10000.0)
    (switch `string` _keytag
      (:`CyanKey`
        (`/Game/Blueprints/OldButUseful/DoorOpener.Cyan` _opener))
      (:`OrangeKey`
        (`/Game/Blueprints/OldButUseful/DoorOpener.Orange` _opener))
      (:`GreenKey`
        (`/Game/Blueprints/OldButUseful/DoorOpener.Green` _opener))
      (:`PurpleKey`
        (`/Game/Blueprints/OldButUseful/DoorOpener.Purple` _opener)))))

(fn `UserConstructionScript`)