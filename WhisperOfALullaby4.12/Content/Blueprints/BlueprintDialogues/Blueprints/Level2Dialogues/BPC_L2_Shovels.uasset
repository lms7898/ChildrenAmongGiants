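; Dialogue component for Level 2 shovel pickups, overriding the dialogue lookups to read rows from the DT_L2_Shovels data table.
; On Use it starts dialogue from the initial branch, unless any shovel dialogue component on the same owner already has an active UI.
; Each use also reports its shovel index to the ShovelManager and registers the owner there, leaving the manager to destroy the shovel.
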(event `/Game/Blueprints/BlueprintDialogues/UseSystem/Blueprints/Interfaces/BPI_Usable.Use`
  (params (PC :type "PlayerController Object Reference"))
  (bind _variable (`|TemporaryVariable`))
  ;[1 1 1] Dialogue
  ;;[1 1 1] Don't spawn a second UI
  (`/Engine/EditorBlueprintResources/StandardMacros.IsValid` (`self.ActiveUI`)
    (:`Is Valid`
      _)
    (:`Is Not Valid`
      (`|AssignmentStatement` _variable)
      (for _array_element (`Actor.K2_GetComponentsByClass` (`self.GetOwner`) "BPC_L2_Shovels_C")
        (`/Engine/EditorBlueprintResources/StandardMacros.IsValid` _array_element
          (:`Is Valid`
            (`/Engine/EditorBlueprintResources/StandardMacros.IsValid` (`/Game/Blueprints/BlueprintDialogues/Blueprints/BPC_Dialogue.ActiveUI` _array_element)
              (:`Is Valid`
                (`|AssignmentStatement` _variable true)
                (break))))))
      (if (not _variable)
        (bind _flow (`self.GetNextState` (`self.InitialBranch`)))
        (`self.SetState` _flow false PC))))
  ;[1 1 1] Store key value
  (`KismetSystemLibrary.PrintString` "shovel get" false true (struct :`R` 0.755 :`B` 0.546502 :`A` 1.0))
  (bind _outactors (`GameplayStatics.GetAllActorsOfClass` "/Game/Blueprints/Utility/ShovelManager.ShovelManager_C"))
  (`/Game/Blueprints/Utility/ShovelManager.ShovelGet` (`KismetArrayLibrary.Array_Get` _outactors) (`self.ShovelIndex`))
  ;[1 1 1] Let shovel manager destroy shovel
  (bind _outactors_2 (`GameplayStatics.GetAllActorsOfClass` "/Game/Blueprints/Utility/ShovelManager.ShovelManager_C"))
  (set `/Game/Blueprints/Utility/ShovelManager.ShovelDialogueOwner` (`self.GetOwner`) (`KismetArrayLibrary.Array_Get` _outactors_2)))

(fn `GetDialogueItem`
  (params (ItemName :type Name))
  (returns (Item :type "/Game/Blueprints/BlueprintDialogues/Blueprints/Structures/Dialogue_TableItem Structure") (Found :type Boolean))
  ;[1 0 1] Override this function for derived classes using another data table
  (bind _returnvalue (`|GetDataTableRow` "/Game/Blueprints/BlueprintDialogues/Data/L2_Dialogues/DT_L2_Shovels.DT_L2_Shovels" ItemName)
    (:`then`
      (bind _result (`/Game/Blueprints/BlueprintDialogues/Utilities/Blueprints/Libs/Lib_Object_UtilityMacros.MakeBoolFromBranch` :!label _label))
      (return _returnvalue _result))
    (:`RowNotFound`
      (goto _label :!via `False`))))

(fn `GetDialogueRowNames`
  (returns (Names :type "Array of Name"))
  ;[1 0 1] Override this function for derived classes using another data table
  (bind _outrownames (`DataTableFunctionLibrary.GetDataTableRowNames` "/Game/Blueprints/BlueprintDialogues/Data/L2_Dialogues/DT_L2_Shovels.DT_L2_Shovels"))
  (return _outrownames))

(fn `GetScriptInterpreter`
  (returns (Interpreter :type "/Game/Blueprints/BlueprintDialogues/ScriptSystem/Blueprints/BP_ScriptInterpreter Object Reference"))
  (return (`/Game/GameModes/ThirdPersonGameMode.SciptInterp` (cast `/Game/GameModes/ThirdPersonGameMode` (`GameplayStatics.GetGameMode`) :!pure true))))