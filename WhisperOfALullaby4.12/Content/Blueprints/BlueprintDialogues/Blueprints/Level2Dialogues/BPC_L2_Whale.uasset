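; Dialogue component for the whale in Level 2, supplying its dialogue lines from the DT_L2_Whale data table.
; It overrides the row lookup and row-name functions so derived dialogue logic reads this table, reporting whether a requested row exists.
; It also fetches the script interpreter from the ThirdPersonGameMode.
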(fn `GetDialogueItem`
  (params (ItemName :type Name))
  (returns (Item :type "/Game/Blueprints/BlueprintDialogues/Blueprints/Structures/Dialogue_TableItem Structure") (Found :type Boolean))
  ;[1 0 1] Override this function for derived classes using another data table
  (bind _returnvalue (`|GetDataTableRow` "/Game/Blueprints/BlueprintDialogues/Data/L2_Dialogues/DT_L2_Whale.DT_L2_Whale" ItemName)
    (:`then`
      (bind _result (`/Game/Blueprints/BlueprintDialogues/Utilities/Blueprints/Libs/Lib_Object_UtilityMacros.MakeBoolFromBranch` :!label _label))
      (return _returnvalue _result))
    (:`RowNotFound`
      (goto _label :!via `False`))))

(fn `GetDialogueRowNames`
  (returns (Names :type "Array of Name"))
  ;[1 0 1] Override this function for derived classes using another data table
  (bind _outrownames (`DataTableFunctionLibrary.GetDataTableRowNames` "/Game/Blueprints/BlueprintDialogues/Data/L2_Dialogues/DT_L2_Whale.DT_L2_Whale"))
  (return _outrownames))

(fn `GetScriptInterpreter`
  (returns (Interpreter :type "/Game/Blueprints/BlueprintDialogues/ScriptSystem/Blueprints/BP_ScriptInterpreter Object Reference"))
  (return (`/Game/GameModes/ThirdPersonGameMode.SciptInterp` (cast `/Game/GameModes/ThirdPersonGameMode` (`GameplayStatics.GetGameMode`) :!pure true))))