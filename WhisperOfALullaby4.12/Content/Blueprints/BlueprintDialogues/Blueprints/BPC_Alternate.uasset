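; BPC_Alternate is a dialogue component that picks its starting branch by input device and reads its lines from DT_DemoDialogue.
; Each tick it reads the game instance's input type and sets the matching type and InitialBranch for mouse/keyboard or Xbox 360.
; Overridable getters supply rows and row names from the table; their level-name switches currently do nothing.
; The script interpreter comes from ThirdPersonGameMode.
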(event `self.ReceiveTick`
  (params (DeltaSeconds :type "Float (single-precision)"))
  (bind _aswoa_lgame_instance (cast `/Game/GameInstances/WoaLGameInstance` (`GameplayStatics.GetGameInstance`)))
  (switch `/Game/GameInstances/InputType` (`/Game/GameInstances/WoaLGameInstance.InputType` _aswoa_lgame_instance)
    (:`NewEnumerator0`
      (`self.SetInputType` "NewEnumerator0")
      (set `self.InitialBranch` "MK_1"))
    (:`NewEnumerator1`
      (`self.SetInputType` "NewEnumerator1")
      (set `self.InitialBranch` "XB360_1"))))

(fn `GetDialogueItem`
  (params (ItemName :type Name))
  (returns (Item :type "/Game/Blueprints/BlueprintDialogues/Blueprints/Structures/Dialogue_TableItem Structure") (Found :type Boolean))
  ;[1 0 1] Override this function for derived classes using another data table
  (bind _returnvalue (`GameplayStatics.GetCurrentLevelName` true))
  (switch `string` _returnvalue
    (:`Default`
      _)
    (:`Town`
      _))
  (bind _returnvalue_2 (`|GetDataTableRow` "/Game/Blueprints/BlueprintDialogues/Data/DT_DemoDialogue.DT_DemoDialogue" ItemName)
    (:`then`
      (bind _result (`/Game/Blueprints/BlueprintDialogues/Utilities/Blueprints/Libs/Lib_Object_UtilityMacros.MakeBoolFromBranch` :!label _label))
      (return _returnvalue_2 _result))
    (:`RowNotFound`
      (goto _label :!via `False`))))

(fn `GetDialogueRowNames`
  (returns (Names :type "Array of Name"))
  ;[1 0 1] Override this function for derived classes using another data table
  (bind _returnvalue (`GameplayStatics.GetCurrentLevelName` true))
  (switch `string` _returnvalue
    (:`Default`
      _)
    (:`Town`
      _))
  (bind _outrownames (`DataTableFunctionLibrary.GetDataTableRowNames` "/Game/Blueprints/BlueprintDialogues/Data/DT_DemoDialogue.DT_DemoDialogue"))
  (return _outrownames))

(fn `GetScriptInterpreter`
  (returns (Interpreter :type "/Game/Blueprints/BlueprintDialogues/ScriptSystem/Blueprints/BP_ScriptInterpreter Object Reference"))
  (return (`/Game/GameModes/ThirdPersonGameMode.SciptInterp` (cast `/Game/GameModes/ThirdPersonGameMode` (`GameplayStatics.GetGameMode`) :!pure true))))