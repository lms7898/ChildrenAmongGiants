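; BPC_KeyDialogue is a dialogue component for a key pickup, with its lines stored in DT_KeyDialogue.
; Its lookup functions return the table's row names and fetch items by name.
; Use reports the key to the first KeyManager found in the level through KeyGet with a fixed index, then destroys the owning actor.
; A helper macro checks whether any BPC_Dialogue component on the owner has an active UI.
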(event `/Game/Blueprints/BlueprintDialogues/UseSystem/Blueprints/Interfaces/BPI_Usable.Use`
  (params (PC :type "PlayerController Object Reference"))
  (`KismetSystemLibrary.PrintString` "key get" false true (struct :`R` 0.755 :`B` 0.546502 :`A` 1.0))
  (bind _outactors (`GameplayStatics.GetAllActorsOfClass` "/Game/Blueprints/Utility/KeyManager.KeyManager_C"))
  (`/Game/Blueprints/Utility/KeyManager.KeyGet` (`KismetArrayLibrary.Array_Get` _outactors) 0)
  (`Actor.K2_DestroyActor` (`self.GetOwner`)))

(fn `GetDialogueItem`
  (params (ItemName :type Name))
  (returns (Item :type "/Game/Blueprints/BlueprintDialogues/Blueprints/Structures/Dialogue_TableItem Structure") (Found :type Boolean))
  (bind _returnvalue (`|GetDataTableRow` "/Game/Blueprints/BlueprintDialogues/Data/L1_Dialogues/DT_KeyDialogue.DT_KeyDialogue" ItemName)
    (:`then`
      (bind _result (`/Game/Blueprints/BlueprintDialogues/Utilities/Blueprints/Libs/Lib_Object_UtilityMacros.MakeBoolFromBranch` :!label _label))
      (return _returnvalue _result))
    (:`RowNotFound`
      (goto _label :!via `False`))))

(fn `GetDialogueRowNames`
  (returns (Names :type "Array of Name"))
  (bind _outrownames (`DataTableFunctionLibrary.GetDataTableRowNames` "/Game/Blueprints/BlueprintDialogues/Data/L1_Dialogues/DT_KeyDialogue.DT_KeyDialogue"))
  (return _outrownames))