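; BPC_ExampleDialogue is an example dialogue component that adapts its starting branch to the player's input device.
; Every Tick it reads the input type from WoaLGameInstance, calls SetInputType and sets InitialBranch to the mouse-keyboard or Xbox 360 branch.
; GetScriptInterpreter supplies the script interpreter held by ThirdPersonGameMode.
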(event `self.ReceiveTick`
  (params (DeltaSeconds :type "Float (single-precision)"))
  (bind _aswoa_lgame_instance (cast `/Game/GameInstances/WoaLGameInstance` (`GameplayStatics.GetGameInstance`)))
  (switch `/Game/GameInstances/InputType` (`/Game/GameInstances/WoaLGameInstance.InputType` _aswoa_lgame_instance)
    (:`NewEnumerator0`
      (`self.SetInputType` "NewEnumerator0")
      (set `self.InitialBranch` "MK_1"))
    (:`NewEnumerator1`
      (`self.SetInputType` "NewEnumerator1")
      (set `self.InitialBranch` "XB360_1"))))

(fn `GetScriptInterpreter`
  (returns (Interpreter :type "/Game/Blueprints/BlueprintDialogues/ScriptSystem/Blueprints/BP_ScriptInterpreter Object Reference"))
  (return (`/Game/GameModes/ThirdPersonGameMode.SciptInterp` (cast `/Game/GameModes/ThirdPersonGameMode` (`GameplayStatics.GetGameMode`) :!pure true))))