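; Dialogue component for orphanage doors that serves dialogue rows from the DT_OrphanageDoors data table.
; On Use, it moves to the next state from the initial branch, unless its own UI or a sibling key-dialogue component's UI is already active.
; It supplies row names, item lookups and the game mode's script interpreter, plus a macro that checks the owner's dialogue components for active UI.
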(event `/Game/Blueprints/BlueprintDialogues/UseSystem/Blueprints/Interfaces/BPI_Usable.Use`
  (params (PC :type "PlayerController Object Reference"))
  (bind _variable (`|TemporaryVariable`))
  ;[1 1 1] Dialogue
  ;;[1 1 1] Don't spawn a second UI
  (`/Engine/EditorBlueprintResources/StandardMacros.IsValid` (`self.ActiveUI`)
    (:`Is Valid`)
    (:`Is Not Valid`
      (`|AssignmentStatement` _variable)
      (for _array_element (`Actor.K2_GetComponentsByClass` (`self.GetOwner`) "/Game/Blueprints/BlueprintDialogues/Blueprints/BPC_KeyDialogue.BPC_KeyDialogue_C")
        (`/Engine/EditorBlueprintResources/StandardMacros.IsValid` _array_element
          (:`Is Valid`
            (`/Engine/EditorBlueprintResources/StandardMacros.IsValid` (`/Game/Blueprints/BlueprintDialogues/Blueprints/BPC_Dialogue.ActiveUI` _array_element)
              (:`Is Valid`
                (`|AssignmentStatement` _variable true)
                (break))))))
      (if (not _variable)
        (bind _flow (`self.GetNextState` (`self.InitialBranch`)))
        (`self.SetState` _flow false PC)))))

(fn `GetDialogueItem`
  (params (ItemName :type Name))
  (returns (Item :type "/Game/Blueprints/BlueprintDialogues/Blueprints/Structures/Dialogue_TableItem Structure") (Found :type Boolean))
  (bind _returnvalue (`|GetDataTableRow` "/Game/Blueprints/BlueprintDialogues/Data/L1_Dialogues/DT_OrphanageDoors.DT_OrphanageDoors" ItemName)
    (:`then`
      (bind _result (`/Game/Blueprints/BlueprintDialogues/Utilities/Blueprints/Libs/Lib_Object_UtilityMacros.MakeBoolFromBranch` :!label _label))
      (return _returnvalue _result))
    (:`RowNotFound`
      (goto _label :!via `False`))))

(fn `GetDialogueRowNames`
  (returns (Names :type "Array of Name"))
  (bind _outrownames (`DataTableFunctionLibrary.GetDataTableRowNames` "/Game/Blueprints/BlueprintDialogues/Data/L1_Dialogues/DT_OrphanageDoors.DT_OrphanageDoors"))
  (return _outrownames))

(fn `GetScriptInterpreter`
  (returns (Interpreter :type "/Game/Blueprints/BlueprintDialogues/ScriptSystem/Blueprints/BP_ScriptInterpreter Object Reference"))
  (return (`/Game/GameModes/ThirdPersonGameMode.SciptInterp` (cast `/Game/GameModes/ThirdPersonGameMode` (`GameplayStatics.GetGameMode`) :!pure true))))