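; Elliana beach follower NPC that trails the player while facing them.
; Every Tick, it issues a SimpleMoveToLocation through its controller toward a point a fixed distance behind the player, derived from the player's forward vector.
; It then snaps its full actor rotation to look at the player with FindLookAtRotation, with no interpolation or axis filtering.
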(event `self.ReceiveTick`
  (params (DeltaSeconds :type "Float (single-precision)"))
  (bind _returnvalue (`GameplayStatics.GetPlayerCharacter` 0))
  (bind _returnvalue_2 (`self.K2_GetActorLocation` _returnvalue))
  (`NavigationSystem.SimpleMoveToLocation` (`self.GetController`) (+ (* (* (`self.GetActorForwardVector` _returnvalue) -1) 200) _returnvalue_2))
  (`self.K2_SetActorRotation` (`KismetMathLibrary.FindLookAtRotation` (`self.K2_GetActorLocation`) _returnvalue_2)))

(fn `UserConstructionScript`)