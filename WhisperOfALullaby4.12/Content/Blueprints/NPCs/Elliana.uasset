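; Elliana is an NPC kid Blueprint that can turn into a moving ball of light and back, currently triggered by test timers on BeginPlay.
; TransformToLight plays an attached particle effect, spawns a TransformedChild light ball, starts its lerp move and hides the skeletal mesh.
; TransformFromLight moves the kid to the ball's XY, keeping her Z, plays a tinted effect, destroys the ball and reveals the mesh after a short delay.
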(event `self.ReceiveBeginPlay`
  ;[1 1 1] Temporarily testing the transform to light function
  (`KismetSystemLibrary.K2_SetTimer` null "TransformToLight" 1.0)
  (`KismetSystemLibrary.K2_SetTimer` null "TransformFromLight" 6.0))

(fn `DisplayMesh`
  ;[1 1 1] ShowTheMesh
  (`SceneComponent.SetVisibility` (`self.SkeletalMeshComponent`) true false))

(fn `TransformFromLight`
  (bind (_returnvalue_x _returnvalue_y _returnvalue_z) (`KismetMathLibrary.BreakVector` (`self.K2_GetActorLocation`)))
  (bind (_returnvalue_x_2 _returnvalue_y_2) (`KismetMathLibrary.BreakVector` (`self.K2_GetActorLocation` (`self.LightBall`))))
  ;[1 1 1] MoveToCorrectPosition
  (`self.K2_SetActorLocation` (`KismetMathLibrary.MakeVector` _returnvalue_x_2 _returnvalue_y_2 _returnvalue_z))
  ;[1 1 1] Spawn the Transformation particle at the kid's center
  (bind _returnvalue (`GameplayStatics.SpawnEmitterAttached` "/Game/Particles/Transform/UnTransform.UnTransform" (`self.SkeletalMeshComponent`) "None" (0.0 0.0 50.0)))
  (`ParticleSystemComponent.SetActorParameter` _returnvalue "Kid" self)
  (`ParticleSystemComponent.SetVectorParameter` _returnvalue "InstanceColorScaleOverLife" (1.0 0.5 0.5))
  (`ParticleSystemComponent.SetFloatParameter` _returnvalue "InstanceAlphaScaleOver" 1.0)
  ;[1 1 1] DestroyLightBall
  (`self.K2_DestroyActor` (`self.LightBall`))
  (`KismetSystemLibrary.K2_SetTimer` null "DisplayMesh" 0.19))

(fn `TransformToLight`
  (bind _returnvalue_location (`KismetMathLibrary.BreakTransform` (`self.GetTransform`)))
  ;[1 1 1] Spawn the Transformation particle at the kid's center
  (bind _returnvalue (`GameplayStatics.SpawnEmitterAttached` "/Game/Particles/Transform/Transform.Transform" (`self.SkeletalMeshComponent`) "None" (0.0 0.0 50.0)))
  (`ParticleSystemComponent.SetActorParameter` _returnvalue "Kid" self)
  ;[1 1 1] Create and move light ball to a new location
  (bind _returnvalue_2 (`|SpawnActorFromClass` "/Game/Blueprints/NPCs/TransformedChild.TransformedChild_C" (`KismetMathLibrary.MakeTransform` (+ _returnvalue_location (0.0 0.0 50.0))) "AlwaysSpawn" "OverrideRootScale"))
  (bind _output_get (set `self.LightBall` _returnvalue_2))
  (`/Game/Blueprints/NPCs/TransformedChild.StartLERP` _output_get (0.0 0.0 300.0) 3.0 0.0 3.0)
  ;[1 1 1] Hide the mesh instantly
  (`SceneComponent.SetVisibility` (`self.SkeletalMeshComponent`) false false))

(fn `UserConstructionScript`)