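; ChildLight is a component for child NPC skeletal mesh actors that turns the kid into a ball of light.
; TransformToLight attaches a transformation particle to the mesh, spawns a TransformedChild light ball, starts its delayed lerp toward Target and hides the mesh.
; Tick keeps the ball's lerp end synced to Target, which follows the player's location while GoToDusk is set.
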(event `self.ReceiveTick`
  (params (DeltaSeconds :type "Float (single-precision)"))
  (if (`KismetSystemLibrary.IsValid` (`self.LightBall`))
    ;[1 1 1] update light target
    (set `/Game/Blueprints/NPCs/TransformedChild.LERP_End` (`self.Target`) (`self.LightBall`)))
  ;[1 1 1] Go to dusk
  (if (`self.GoToDusk`)
    (set `self.Target` (`Actor.K2_GetActorLocation` (`GameplayStatics.GetPlayerCharacter` 0)))))

(fn `TransformToLight`
  ;[1 1 1] Spawn the Transformation particle at the kid's center
  (bind _asskeletal_mesh_actor (cast `SkeletalMeshActor` (`self.GetOwner`)))
  (set `self.SkeletalMesh` (`SkeletalMeshActor.SkeletalMeshComponent` _asskeletal_mesh_actor))
  (bind _returnvalue (`GameplayStatics.SpawnEmitterAttached` "/Game/Particles/Transform/Transform.Transform" (`self.SkeletalMesh`) "None" (0.0 0.0 50.0)))
  (`ParticleSystemComponent.SetActorParameter` _returnvalue "Kid" (`self.GetOwner`))
  ;[1 1 1] Create and move light ball to a new location
  (bind _returnvalue_2 (`|SpawnActorFromClass` "/Game/Blueprints/NPCs/TransformedChild.TransformedChild_C" (`KismetMathLibrary.MakeTransform` (+ (`Actor.K2_GetActorLocation` (`self.GetOwner`)) (0.0 0.0 50.0))) "AlwaysSpawn" "OverrideRootScale"))
  (bind _output_get (set `self.LightBall` _returnvalue_2))
  (`/Game/Blueprints/NPCs/TransformedChild.StartLERP` _output_get (`self.Target`) 1.0 0.0 2.7)
  ;[1 1 1] Hide the mesh instantly
  (`SceneComponent.SetVisibility` (`self.SkeletalMesh`) false false))