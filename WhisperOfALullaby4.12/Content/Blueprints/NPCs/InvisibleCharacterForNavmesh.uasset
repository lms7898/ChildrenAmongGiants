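; Invisible navmesh character that walks to given locations and notifies Elliana on arrival during her house search.
; MoveToLocationWithCallback stores the destination, starts a SimpleMoveToLocation through its controller and flags it as en route.
; Tick polls squared distance to the destination and, once close enough, clears the flag and calls BeginNextHouseSearchSegment on the Elliana actor found at BeginPlay.
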(event `self.ReceiveBeginPlay`
  ;[1 1 1] Elli ref
  (bind _outactors (`GameplayStatics.GetAllActorsOfClass` "/Game/Blueprints/NPCs/Elliana.Elliana_C"))
  (set `self.Elli` (`KismetArrayLibrary.Array_Get` _outactors)))

(event `self.ReceiveTick`
  (params (DeltaSeconds :type "Float (single-precision)"))
  ;[1 1 1] Check if arrived
  (if (`self.EnRoute`)
    (if (< (`KismetMathLibrary.VSizeSquared` (- (`self.Destination`) (`self.K2_GetActorLocation`))) 100000.0)
      (set `self.EnRoute` false)
      (`/Game/Blueprints/NPCs/Elliana.BeginNextHouseSearchSegment` (`self.Elli`)))))

(fn `MoveToLocationWithCallback`
  (params (Location :type "Vector Structure"))
  (bind _output_get (set `self.Destination` Location))
  (`NavigationSystem.SimpleMoveToLocation` (`self.GetController`) _output_get)
  (set `self.EnRoute` true))

(fn `UserConstructionScript`)