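; BPC_L2_ThroneRoom supplies the dialogue data for the Level 2 throne room cutscene.
; It overrides the dialogue lookup functions to read rows and row names from DT_ThroneRoomCutscene, with a found flag on item lookups.
; It also gets the script interpreter from ThirdPersonGameMode.
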(fn `GetDialogueItem`
  (params (ItemName :type Name))
  (returns (Item :type "/Game/Blueprints/BlueprintDialogues/Blueprints/Structures/Dialogue_TableItem Structure") (Found :type Boolean))
  ;[1 0 1] Override this function for derived classes using another data table
  (bind _returnvalue (`|GetDataTableRow` "/Game/Cutscenes/Level2/Beach/ThroneRoom/DT_ThroneRoomCutscene.DT_ThroneRoomCutscene" ItemName)
    (:`then`
      (bind _result (`/Game/Blueprints/BlueprintDialogues/Utilities/Blueprints/Libs/Lib_Object_UtilityMacros.MakeBoolFromBranch` :!label _label))
      (return _returnvalue _result))
    (:`RowNotFound`
      (goto _label :!via `False`))))

(fn `GetDialogueRowNames`
  (returns (Names :type "Array of Name"))
  ;[1 0 1] Override this function for derived classes using another data table
  (bind _outrownames (`DataTableFunctionLibrary.GetDataTableRowNames` "/Game/Cutscenes/Level2/Beach/ThroneRoom/DT_ThroneRoomCutscene.DT_ThroneRoomCutscene"))
  (return _outrownames))

(fn `GetScriptInterpreter`
  (returns (Interpreter :type "/Game/Blueprints/BlueprintDialogues/ScriptSystem/Blueprints/BP_ScriptInterpreter Object Reference"))
  (return (`/Game/GameModes/ThirdPersonGameMode.SciptInterp` (cast `/Game/GameModes/ThirdPersonGameMode` (`GameplayStatics.GetGameMode`) :!pure true))))