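; Checkpoint actor that sets the player's respawn location when the ThirdPersonCharacter overlaps it.
; On overlap it writes its own transform to SpawnTransform on ThirdPersonGameMode, deactivates the character's previous ActiveCheckpoint, then registers and activates itself.
; Activate and Deactivate toggle visibility between active and inactive particle components, so the current checkpoint is visually marked.
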(event `self.ReceiveActorBeginOverlap`
  (params (OtherActor :type "Actor Object Reference"))
  (bind _returnvalue (`GameplayStatics.GetGameMode`))
  (if (== (`GameplayStatics.GetObjectClass` OtherActor) "/Game/Blueprints/ThirdPersonCharacter.ThirdPersonCharacter_C")
    (if (== (`GameplayStatics.GetObjectClass` _returnvalue) "/Game/GameModes/ThirdPersonGameMode.ThirdPersonGameMode_C")
      (bind _asthird_person_game_mode (cast `/Game/GameModes/ThirdPersonGameMode` _returnvalue))
      (set `/Game/GameModes/ThirdPersonGameMode.Spawn Transform` (`self.GetTransform`) _asthird_person_game_mode)
      (bind _asthird_person_character (cast `/Game/Blueprints/ThirdPersonCharacter` OtherActor))
      (`self.Deactivate` (`/Game/Blueprints/ThirdPersonCharacter.ActiveCheckpoint` _asthird_person_character))
      (bind _output_get (set `/Game/Blueprints/ThirdPersonCharacter.ActiveCheckpoint` self _asthird_person_character))
      (`self.Activate` _output_get))))

(fn `Activate`
  (`SceneComponent.SetVisibility` (`self.DeactiveParticles`) false false)
  (`SceneComponent.SetVisibility` (`self.ActiveParticles`) true false))

(fn `Deactivate`
  (`SceneComponent.SetVisibility` (`self.DeactiveParticles`) true false)
  (`SceneComponent.SetVisibility` (`self.ActiveParticles`) false false))

(fn `UserConstructionScript`)