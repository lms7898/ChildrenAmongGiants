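; DummyOrbRotate is an orb actor that gives off a fading burst of light on the Illuminate input.
; When unlit, a press plays a magic sound, activates particles, maxes the point light and sets ThirdPersonCharacter's Illuminating flag.
; A Delay loop steps intensity down to zero, then clears the flag.
; Tick, throttled by a Delay, repeatedly enables player input and the sphere's custom depth rendering.
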(event `InputAction|Illuminate`
  (params (Key :type "Key Structure" :default "AnyKey"))
  (bind _pointlight (`self.PointLight`))
  (bind _intensity (`LightComponentBase.Intensity` _pointlight))
  (:`Pressed`
    (bind _asthird_person_character (cast `/Game/Blueprints/ThirdPersonCharacter` (`GameplayStatics.GetPlayerCharacter` 0)))
    (if (not (> (`LightComponentBase.Intensity` _pointlight) 0.0))
      (`GameplayStatics.PlaySound2D` "/Game/Audio/Magic1_Cue.Magic1_Cue")
      (`LightComponent.SetIntensity` _pointlight 20000.0)
      (`ActorComponent.Activate` (`self.ParticleSystem`) true)
      (set `/Game/Blueprints/ThirdPersonCharacter.Illuminating?` true _asthird_person_character))
    (`LightComponent.SetIntensity` _pointlight (- _intensity 200.0) :!label _label)
    (`KismetSystemLibrary.Delay` 0.001)
    (if (> _intensity 0.0)
      (goto _label)
      (else
        (`LightComponent.SetIntensity` _pointlight 0.0)
        (set `/Game/Blueprints/ThirdPersonCharacter.Illuminating?` false _asthird_person_character)))))

(event `self.ReceiveTick`
  (params (DeltaSeconds :type "Float (single-precision)"))
  (`KismetSystemLibrary.Delay` 1.0)
  (`PrimitiveComponent.SetRenderCustomDepth` (`self.Sphere`) true)
  (`self.EnableInput` (`GameplayStatics.GetPlayerController` 0)))

(fn `UserConstructionScript`)