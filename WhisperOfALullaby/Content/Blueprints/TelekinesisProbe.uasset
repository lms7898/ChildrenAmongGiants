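; TelekinesisProbe is an overlap probe that makes movable objects glow, apparently marking candidates for telekinesis.
; On begin overlap it takes the other actor's first StaticMeshComponent and, if its mass is below a fixed limit, enables Render Custom Depth.
; End overlap repeats the same checks and disables it.
; The Blueprint only toggles that flag and contains no logic for moving objects.
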(event `self.ReceiveActorEndOverlap`
  (params (OtherActor :type "Actor Object Reference"))
  (bind _item (`KismetArrayLibrary.Array_Get` (`self.K2_GetComponentsByClass` OtherActor "/Script/Engine.StaticMeshComponent")))
  ;[1 1 1] Movable Objects Glow
  (if (`KismetSystemLibrary.IsValid` _item)
    (if (< (`PrimitiveComponent.GetMass` _item) 500.0)
      ;;[1 1 1] Magic Happens Here
      (`PrimitiveComponent.SetRenderCustomDepth` _item false))))

(event `self.ReceiveActorBeginOverlap`
  (params (OtherActor :type "Actor Object Reference"))
  (bind _item (`KismetArrayLibrary.Array_Get` (`self.K2_GetComponentsByClass` OtherActor "/Script/Engine.StaticMeshComponent")))
  ;[1 1 1] Movable Objects Glow
  (if (`KismetSystemLibrary.IsValid` _item)
    (if (< (`PrimitiveComponent.GetMass` _item) 500.0)
      ;;[1 1 1] Magic Happens Here
      (`PrimitiveComponent.SetRenderCustomDepth` _item true))))

(fn `UserConstructionScript`)