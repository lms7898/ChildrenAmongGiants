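; Crowd character Blueprint that wanders between randomly chosen TargetPoints using SimpleMoveToActor.
; Tick destroys it below zero height; when nearly stationary, it picks a new waypoint and moves, or teleports to a reset strip after a second stuck.
; Any actor overlap also picks a new waypoint and marks it on the ground floor.
; Escalator nodes are gathered, but top-floor handling is empty, and player-chase and debug logic are disconnected.
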(event `self.ReceiveBeginPlay`
  (bind _targetpoints (`self.TargetPoints`))
  ;[1 1 1] On Start
  ;;[1 1 1] Get The List of Waypoints
  (bind _outactors (`GameplayStatics.GetAllActorsOfClass` "/Script/Engine.TargetPoint"))
  (bind _output_get (set `self.TargetPoints` _outactors))
  (set `self.CurrentTarget` (`KismetArrayLibrary.Array_Get` _output_get))
  ;;[1 1 1] Get Reference To Escalator Points
  (bind _outactors_2 (`GameplayStatics.GetAllActorsOfClass` "/Game/Blueprints/EscalatorNode.EscalatorNode_C"))
  (set `self.escalatorNodes` _outactors_2)
  ;;[1 1 1] Start on Ground Floor
  (set `self.groundfloor` true)
  (set `self.lastMovement` (`KismetSystemLibrary.GetGameTimeInSeconds`))
  ;[1 1 1] Get First Target Point
  (set `self.currentTarget` (`KismetArrayLibrary.Array_Get` _targetpoints (`KismetMathLibrary.RandomInteger` (`KismetArrayLibrary.Array_Length` _targetpoints)))))

(event `ReplaceWithCrowd`
  ;[1 1 1] Stop chasing after 10 seconds
)

(event `self.ReceiveActorBeginOverlap`
  (params (OtherActor :type "Actor Object Reference"))
  ;[1 1 1] If you are in the reset box, get a new target
  (`self.SetRandomWaypoint`)
  (set `self.groundfloor` true))

(event `self.ReceiveTick`
  (params (DeltaSeconds :type "Float (single-precision)"))
  (bind _returnvalue (`KismetSystemLibrary.GetGameTimeInSeconds`))
  ;[1 1 1] Tick
  ;[1 1 1] Out of bounds
  (if (< (.z (.location (`self.GetTransform`))) 0.0)
    (`self.K2_DestroyActor`)
    (else
      ;[1 1 1] If Character is not moving
      (if (< (`KismetMathLibrary.VSize` (`MovementComponent.Velocity` (`self.CharacterMovement`))) 1.0)
        ;[1 1 1] If Stuck, Forget Escalator
        (set `self.MovementLocked` false)
        ;[1 1 1] If Stuck, Set New Waypoint
        (`self.SetRandomWaypoint`)
        ;[1 1 1] Check Permanently Stuck
        (if (> (- _returnvalue (`self.lastMovement`)) 1.0)
          ;[1 1 1] If permanently stuck, reset
          (`self.K2_SetActorLocation` (`KismetMathLibrary.MakeVector` -2000.0 (* (`KismetMathLibrary.RandomFloat`) 1000.0) 140.0) false true)
          (set `self.MovementLocked` false)
          (set `self.lastMovement` (`KismetSystemLibrary.GetGameTimeInSeconds`))
          (else
            ;[1 1 1] Walk
            (`NavigationSystem.SimpleMoveToActor` (`self.GetController`) (`self.currentTarget`))))
        (else
          (set `self.lastMovement` _returnvalue)
          ;[1 1 1] Check if the character is already on an escalator
          (if (not (`self.MovementLocked`))
            ;[1 1 1] If the character is targeting the topfloor
            (if (`ActorComponent.ComponentHasTag` (`TargetPoint.SpriteComponent` (`self.currentTarget`)) "TopFloor")
              _)))))))

(event `SetRandomWaypoint`
  (bind _targetpoints (`self.TargetPoints`))
  ;[1 1 1] Set New Target Point
  (set `self.currentTarget` (`KismetArrayLibrary.Array_Get` _targetpoints (`KismetMathLibrary.RandomInteger` (`KismetArrayLibrary.Array_Length` _targetpoints)))))

(fn `UserConstructionScript`)