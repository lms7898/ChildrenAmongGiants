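; SaveGameActor is a level actor that initializes save data for five MBElli boolean flags when play begins.
; If the save slot exists, it loads the WoaLSaveGame; otherwise it creates one with all flags false and writes it to the slot.
; Either path copies the flags into WoaLGameInstance, and the actor never saves later changes back.
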(event `self.ReceiveBeginPlay`
  (bind _gameinstanceref (`self.GameInstanceRef`))
  (bind _woalsavegameref (`self.WoaLSaveGameRef`))
  (bind _gameinstanceref_2 (`self.GameInstanceRef`))
  (bind _woalsavegameref_2 (`self.WoaLSaveGameRef`))
  ;[1 1 1] Set Game Instance Ref
  (bind _aswoa_lgame_instance (cast `/Game/GameInstances/WoaLGameInstance` (`GameplayStatics.GetGameInstance`)))
  (set `self.GameInstanceRef` _aswoa_lgame_instance)
  (bind _returnvalue (`GameplayStatics.DoesSaveGameExist` (`self.SaveGameSlot`)))
  (if _returnvalue
    ;[1 1 1] Load Game
    (bind _returnvalue_2 (`GameplayStatics.LoadGameFromSlot` (`self.SaveGameSlot`)))
    (bind _output_get (set `self.BP_SaveGame` _returnvalue_2))
    (bind _aswoa_lsave_game (cast `/Game/Blueprints/SaveState/WoaLSaveGame` _output_get))
    (set `self.WoaLSaveGameRef` _aswoa_lsave_game)
    ;;[1 1 1] Update Game Instance
    (set `/Game/GameInstances/WoaLGameInstance.MBElli1` (`/Game/Blueprints/SaveState/WoaLSaveGame.S_MBElli1` _woalsavegameref) _gameinstanceref)
    (set `/Game/GameInstances/WoaLGameInstance.MBElli2` (`/Game/Blueprints/SaveState/WoaLSaveGame.S_MBElli2` _woalsavegameref) _gameinstanceref)
    (set `/Game/GameInstances/WoaLGameInstance.MBElli3` (`/Game/Blueprints/SaveState/WoaLSaveGame.S_MBElli3` _woalsavegameref) _gameinstanceref)
    (set `/Game/GameInstances/WoaLGameInstance.MBElli4` (`/Game/Blueprints/SaveState/WoaLSaveGame.S_MBElli4` _woalsavegameref) _gameinstanceref)
    (set `/Game/GameInstances/WoaLGameInstance.MBElli5` (`/Game/Blueprints/SaveState/WoaLSaveGame.S_MBElli5` _woalsavegameref) _gameinstanceref)
    (else
      ;[1 1 1] Initial Save
      (bind _returnvalue_3 (`GameplayStatics.CreateSaveGameObject` "/Game/Blueprints/SaveState/WoaLSaveGame.WoaLSaveGame_C"))
      (bind _output_get_2 (set `self.BP_SaveGame` _returnvalue_3))
      (bind _aswoa_lsave_game_2 (cast `/Game/Blueprints/SaveState/WoaLSaveGame` _output_get_2))
      (bind _output_get_3 (set `self.WoaLSaveGameRef` _aswoa_lsave_game_2))
      ;;[1 1 1] Default Values
      (set `/Game/Blueprints/SaveState/WoaLSaveGame.S_MBElli1` false _output_get_3)
      (set `/Game/Blueprints/SaveState/WoaLSaveGame.S_MBElli2` false _output_get_3)
      (set `/Game/Blueprints/SaveState/WoaLSaveGame.S_MBElli3` false _output_get_3)
      (set `/Game/Blueprints/SaveState/WoaLSaveGame.S_MBElli4` false _output_get_3)
      (set `/Game/Blueprints/SaveState/WoaLSaveGame.S_MBElli5` false _output_get_3)
      (`GameplayStatics.SaveGameToSlot` _output_get_3 (`self.SaveGameSlot`))
      ;;[1 1 1] Update Game Instance
      (set `/Game/GameInstances/WoaLGameInstance.MBElli1` (`/Game/Blueprints/SaveState/WoaLSaveGame.S_MBElli1` _woalsavegameref_2) _gameinstanceref_2)
      (set `/Game/GameInstances/WoaLGameInstance.MBElli2` (`/Game/Blueprints/SaveState/WoaLSaveGame.S_MBElli2` _woalsavegameref_2) _gameinstanceref_2)
      (set `/Game/GameInstances/WoaLGameInstance.MBElli3` (`/Game/Blueprints/SaveState/WoaLSaveGame.S_MBElli3` _woalsavegameref_2) _gameinstanceref_2)
      (set `/Game/GameInstances/WoaLGameInstance.MBElli4` (`/Game/Blueprints/SaveState/WoaLSaveGame.S_MBElli4` _woalsavegameref_2) _gameinstanceref_2)
      (set `/Game/GameInstances/WoaLGameInstance.MBElli5` (`/Game/Blueprints/SaveState/WoaLSaveGame.S_MBElli5` _woalsavegameref_2) _gameinstanceref_2))))

(fn `UserConstructionScript`)