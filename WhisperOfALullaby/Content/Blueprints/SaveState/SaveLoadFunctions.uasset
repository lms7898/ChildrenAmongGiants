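; Save/load helper that persists five MBElli boolean flags between the game instance and a save slot.
; SaveGame builds a fresh WoaLSaveGame object, copies the flags from WoaLGameInstance and writes it to the slot.
; LoadGame copies them back into the game instance if the slot exists.
; WipeSave overwrites the slot with all flags false, leaving the live game instance values untouched.
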(fn SaveGame
  ;[1 1 1] Set Game Instance Ref
  (bind _aswoa_lgame_instance (Utilities|Casting|CastToWoaLGameInstance (Game|GetGameInstance)))
  (LocalVariables|SetGameInstanceRef _aswoa_lgame_instance)
  ;[1 1 1] Initial Save
  (bind _returnvalue (SaveGame|CreateSaveGameObject "/Game/Blueprints/SaveState/WoaLSaveGame.WoaLSaveGame_C"))
  (bind _output_get (LocalVariables|SetBP_SaveGame _returnvalue))
  (bind _aswoa_lsave_game (Utilities|Casting|CastToWoaLSaveGame _output_get))
  (bind _output_get_2 (LocalVariables|SetWoaLSaveGameRef _aswoa_lsave_game))
  ;;[1 1 1] Update saved values
  (Variables|/Game/Blueprints/SaveState/WoaLSaveGame.WoaLSaveGame_C|SetS_MBElli1 _output_get_2 (Variables|/Game/GameInstances/WoaLGameInstance.WoaLGameInstance_C|GetMBElli1 (LocalVariables|GetGameInstanceRef)))
  (Variables|/Game/Blueprints/SaveState/WoaLSaveGame.WoaLSaveGame_C|SetS_MBElli2 _output_get_2 (Variables|/Game/GameInstances/WoaLGameInstance.WoaLGameInstance_C|GetMBElli2 (LocalVariables|GetGameInstanceRef)))
  (Variables|/Game/Blueprints/SaveState/WoaLSaveGame.WoaLSaveGame_C|SetS_MBElli3 _output_get_2 (Variables|/Game/GameInstances/WoaLGameInstance.WoaLGameInstance_C|GetMBElli3 (LocalVariables|GetGameInstanceRef)))
  (Variables|/Game/Blueprints/SaveState/WoaLSaveGame.WoaLSaveGame_C|SetS_MBElli4 _output_get_2 (Variables|/Game/GameInstances/WoaLGameInstance.WoaLGameInstance_C|GetMBElli4 (LocalVariables|GetGameInstanceRef)))
  (Variables|/Game/Blueprints/SaveState/WoaLSaveGame.WoaLSaveGame_C|SetS_MBElli5 _output_get_2 (Variables|/Game/GameInstances/WoaLGameInstance.WoaLGameInstance_C|GetMBElli5 (LocalVariables|GetGameInstanceRef)))
  ;;[1 1 1] Save to Slot
  (SaveGame|SaveGametoSlot _output_get_2 (LocalVariables|GetSaveGameSlot)))

(fn LoadGame
  ;[1 1 1] Set Game Instance Ref
  (bind _aswoa_lgame_instance (Utilities|Casting|CastToWoaLGameInstance (Game|GetGameInstance)))
  (LocalVariables|SetGameInstanceRef _aswoa_lgame_instance)
  (bind _returnvalue (SaveGame|DoesSaveGameExist (LocalVariables|GetSaveGameSlot)))
  (if _returnvalue
    ;[1 1 1] Load Game
    (bind _returnvalue_2 (SaveGame|LoadGamefromSlot (LocalVariables|GetSaveGameSlot)))
    (bind _output_get (LocalVariables|SetBP_SaveGame _returnvalue_2))
    (bind _aswoa_lsave_game (Utilities|Casting|CastToWoaLSaveGame _output_get))
    (LocalVariables|SetWoaLSaveGameRef _aswoa_lsave_game)
    ;;[1 1 1] Update Game Instance
    (Variables|/Game/GameInstances/WoaLGameInstance.WoaLGameInstance_C|SetMBElli1 (LocalVariables|GetGameInstanceRef) (Variables|/Game/Blueprints/SaveState/WoaLSaveGame.WoaLSaveGame_C|GetS_MBElli1 (LocalVariables|GetWoaLSaveGameRef)))
    (Variables|/Game/GameInstances/WoaLGameInstance.WoaLGameInstance_C|SetMBElli2 (LocalVariables|GetGameInstanceRef) (Variables|/Game/Blueprints/SaveState/WoaLSaveGame.WoaLSaveGame_C|GetS_MBElli2 (LocalVariables|GetWoaLSaveGameRef)))
    (Variables|/Game/GameInstances/WoaLGameInstance.WoaLGameInstance_C|SetMBElli3 (LocalVariables|GetGameInstanceRef) (Variables|/Game/Blueprints/SaveState/WoaLSaveGame.WoaLSaveGame_C|GetS_MBElli3 (LocalVariables|GetWoaLSaveGameRef)))
    (Variables|/Game/GameInstances/WoaLGameInstance.WoaLGameInstance_C|SetMBElli4 (LocalVariables|GetGameInstanceRef) (Variables|/Game/Blueprints/SaveState/WoaLSaveGame.WoaLSaveGame_C|GetS_MBElli4 (LocalVariables|GetWoaLSaveGameRef)))
    (Variables|/Game/GameInstances/WoaLGameInstance.WoaLGameInstance_C|SetMBElli5 (LocalVariables|GetGameInstanceRef) (Variables|/Game/Blueprints/SaveState/WoaLSaveGame.WoaLSaveGame_C|GetS_MBElli5 (LocalVariables|GetWoaLSaveGameRef)))))

(fn WipeSave
  ;[1 1 1] Initial Save
  (bind _returnvalue (SaveGame|CreateSaveGameObject "/Game/Blueprints/SaveState/WoaLSaveGame.WoaLSaveGame_C"))
  (bind _output_get (LocalVariables|SetBP_SaveGame _returnvalue))
  (bind _aswoa_lsave_game (Utilities|Casting|CastToWoaLSaveGame _output_get))
  (bind _output_get_2 (LocalVariables|SetWoaLSaveGameRef _aswoa_lsave_game))
  ;;[1 1 1] Update saved values
  (Variables|/Game/Blueprints/SaveState/WoaLSaveGame.WoaLSaveGame_C|SetS_MBElli1 _output_get_2 false)
  (Variables|/Game/Blueprints/SaveState/WoaLSaveGame.WoaLSaveGame_C|SetS_MBElli2 _output_get_2 false)
  (Variables|/Game/Blueprints/SaveState/WoaLSaveGame.WoaLSaveGame_C|SetS_MBElli3 _output_get_2 false)
  (Variables|/Game/Blueprints/SaveState/WoaLSaveGame.WoaLSaveGame_C|SetS_MBElli4 _output_get_2 false)
  (Variables|/Game/Blueprints/SaveState/WoaLSaveGame.WoaLSaveGame_C|SetS_MBElli5 _output_get_2 false)
  ;;[1 1 1] Save to Slot
  (SaveGame|SaveGametoSlot _output_get_2 (LocalVariables|GetSaveGameSlot)))