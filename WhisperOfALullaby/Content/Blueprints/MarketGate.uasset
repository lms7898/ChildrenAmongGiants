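; MarketGate is a gate actor that bursts open when the player character overlaps it and the KeyManager allows it.
; Each overlap before launch calls OpenSesame on the KeyManager, then checks its Open flag.
; A one-time launch teleports the actor along negative Y, then flings StaticMesh5 with physics spin and a strong Y velocity.
; It also sets the character mesh's physics velocity to the character's current velocity.
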(event `self.ReceiveActorBeginOverlap`
  (params (OtherActor :type "Actor Object Reference"))
  (bind _keymanager (`self.KeyManager`))
  (bind _staticmesh5 (`self.StaticMesh5`))
  (if (not (`self.Launched`))
    (if (== (`GameplayStatics.GetObjectClass` OtherActor) "/Game/Blueprints/ThirdPersonCharacter.ThirdPersonCharacter_C")
      (`/Game/Blueprints/KeyManager.OpenSesame` _keymanager)
      (if (`/Game/Blueprints/KeyManager.Open` _keymanager)
        (set `self.Launched` true)
        (`self.K2_AddActorWorldOffset` (`KismetMathLibrary.MakeVector` 0.0 -500.0 0.0) false true)
        (`PrimitiveComponent.SetSimulatePhysics` _staticmesh5 true)
        (`PrimitiveComponent.SetPhysicsAngularVelocity` _staticmesh5 (-800.0 0.0 0.0) false "None")
        (`PrimitiveComponent.SetPhysicsLinearVelocity` _staticmesh5 (`KismetMathLibrary.MakeVector` 0.0 (+ (.y (`self.GetVelocity` OtherActor)) 12000.0) (.z (`self.GetVelocity` OtherActor))) false "None")
        (bind _asthird_person_character (cast `/Game/Blueprints/ThirdPersonCharacter` OtherActor))
        (`PrimitiveComponent.SetPhysicsLinearVelocity` (`Character.Mesh` _asthird_person_character) (`self.GetVelocity` OtherActor) false "None")))))

(event `self.ReceiveTick`
  (params (DeltaSeconds :type "Float (single-precision)")))

(fn `UserConstructionScript`)