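; EllianaCharacter is a character Blueprint that travels between indexed target points using navmesh moves or straight-line lerps.
; Events select a point or start a lerp, while Tick issues SimpleMoveToLocation through the AI controller until near the goal.
; Arrival at certain indices triggers lerps to hard-coded locations.
; Lerps teleport the actor each tick, timed by distance over speed, and pause navmesh movement until finished.
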(event `self.ReceiveBeginPlay`
  ;[1 1 1] Start
  (bind _returnvalue (`AIBlueprintHelperLibrary.GetAIController` self))
  (set `self.AI` _returnvalue))

(event `AdvanceTarget`
  ;[1 1 1] Advance target point (navmesh)
  (set `self.PointsIndex` (+ (`self.PointsIndex`) 1))
  (set `self.currentTarget` (`KismetArrayLibrary.Array_Get` (`self.TargetPoints`) (`self.PointsIndex`)))
  (set `self.UseNavMesh` true))

(event `self.ReceiveTick`
  (params (DeltaSeconds :type "Float (single-precision)"))
  (bind _returnvalue (`self.K2_GetActorLocation` (`KismetArrayLibrary.Array_Get` (`self.TargetPoints`) (`self.pointsIndex`))))
  (bind _returnvalue_2 (/ (`KismetMathLibrary.GetTotalMilliseconds` (- (`KismetMathLibrary.Now`) (`self.startTime`))) (`self.duration`)))
  ;[1 1 1] Tick
  (if (`self.LERPing`)
    ;[1 1 1] LERP
    (`self.K2_SetActorLocation` (`KismetMathLibrary.VLerp` (`self.start`) (`self.end`) _returnvalue_2) false true)
    (if (> _returnvalue_2 1.0)
      (set `self.LERPing` false))
    (else
      ;[1 1 1] Use Nav Mesh To Point
      (if (`self.UseNavMesh`)
        (`NavigationSystem.SimpleMoveToLocation` (`self.AI`) _returnvalue)
        (if (< (`KismetMathLibrary.VSizeSquared` (- _returnvalue (`self.K2_GetActorLocation`))) 100000.0)
          (set `self.UseNavMesh` false)
          (`KismetSystemLibrary.PrintString` "Hello")
          (switch `int` (`self.pointsIndex`)
            (:`1`
              (`self.LERPToLocation` (-1540.0 -13350.0 4400.0)))
            (:`2`
              (`self.LERPToLocation` (-1610.0 -13790.0 4400.0)))))))))

(event `LERPToLocation`
  (params (NewLocation :type "Vector Structure") (TargetPoint :type Integer))
  ;[1 1 1] Set LERP Target
  (set `self.end` NewLocation)
  (set `self.start` (`self.K2_GetActorLocation`))
  (set `self.startTime` (`KismetMathLibrary.Now`))
  (set `self.LERPing` true)
  (set `self.duration` (/ (`KismetMathLibrary.VSize` (- (`self.end`) (`self.start`))) (`self.LERPspeed`)))
  ;[1 1 1] Activate Nav Mesh?
  (if (> TargetPoint -1)
    (set `self.pointsIndex` TargetPoint)
    (set `self.UseNavMesh` true)))

(event `GoToTargetPointNum`
  (params (num :type Integer))
  ;[1 1 1] goto target point (navmesh)
  (set `self.PointsIndex` num)
  (set `self.currentTarget` (`KismetArrayLibrary.Array_Get` (`self.TargetPoints`) (`self.PointsIndex`)))
  (set `self.UseNavMesh` true))

(fn `UserConstructionScript`)