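; Dialogue component for cutscenes that sources its lines from the DT_CutsceneDialogue data table.
; Use starts the flow at InitialBranch, unless this component or another BPC_Dialogue on the owner already has an active UI.
; Overridable getters supply rows and row names, with a level-name switch that currently has no per-level behavior.
; It also exposes the script interpreter held by ThirdPersonGameMode.
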(event `/Game/Blueprints/BlueprintDialogues/UseSystem/Blueprints/Interfaces/BPI_Usable.Use`
  (params (PC :type "PlayerController Object Reference"))
  ;[1 1 1] Don't spawn a second UI
  (`self.OwnerHasActiveDialogues`
    (:`false`
      (bind _flow (`self.GetNextState` (`self.InitialBranch`)))
      (`self.SetState` _flow false PC))))

(event `self.OnAllTextDisplayed`)

(fn `GetDialogueItem`
  (params (ItemName :type Name))
  (returns (Item :type "/Game/Blueprints/BlueprintDialogues/Blueprints/Structures/Dialogue_TableItem Structure") (Found :type Boolean))
  ;[1 0 1] Override this function for derived classes using another data table
  (bind _returnvalue (`GameplayStatics.GetCurrentLevelName` true))
  (switch `string` _returnvalue
    (:`Default`
      _)
    (:`Town`
      _))
  (bind _returnvalue_2 (`|GetDataTableRow` "/Game/Blueprints/BlueprintDialogues/Data/DT_CutsceneDialogue.DT_CutsceneDialogue" ItemName)
    (:`then`
      (bind _result (`/Game/Blueprints/BlueprintDialogues/Utilities/Blueprints/Libs/Lib_Object_UtilityMacros.MakeBoolFromBranch` :!label _label))
      (return _returnvalue_2 _result))
    (:`RowNotFound`
      (goto _label :!via `False`))))

(fn `GetDialogueRowNames`
  (returns (Names :type "Array of Name"))
  ;[1 0 1] Override this function for derived classes using another data table
  (bind _returnvalue (`GameplayStatics.GetCurrentLevelName` true))
  (switch `string` _returnvalue
    (:`Default`
      _)
    (:`Town`
      _))
  (bind _outrownames (`DataTableFunctionLibrary.GetDataTableRowNames` "/Game/Blueprints/BlueprintDialogues/Data/DT_CutsceneDialogue.DT_CutsceneDialogue"))
  (return _outrownames))

(fn `GetScriptInterpreter`
  (returns (Interpreter :type "/Game/Blueprints/BlueprintDialogues/ScriptSystem/Blueprints/BP_ScriptInterpreter Object Reference"))
  (return (`/Game/GameModes/ThirdPersonGameMode.SciptInterp` (cast `/Game/GameModes/ThirdPersonGameMode` (`GameplayStatics.GetGameMode`) :!pure true))))