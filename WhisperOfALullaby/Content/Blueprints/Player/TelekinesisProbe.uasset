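; TelekinesisProbe is an overlap probe that highlights physics objects the player could move with telekinesis.
; Overlapping actors whose first static mesh simulates physics and is under a mass limit are added to a candidate array.
; Tick projects each candidate to screen space, enabling custom depth and stencil on those inside the viewport for a glow.
; End overlap disables custom depth but leaves the actor in the array.
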(event `self.ReceiveActorEndOverlap`
  (params (OtherActor :type "Actor Object Reference"))
  (bind _item (`KismetArrayLibrary.Array_Get` (`self.K2_GetComponentsByClass` OtherActor "/Script/Engine.StaticMeshComponent")))
  ;[1 1 1] Movable Objects Glow
  (if (`KismetSystemLibrary.IsValid` _item)
    (if (`SceneComponent.IsAnySimulatingPhysics` _item)
      (if (< (`PrimitiveComponent.GetMass` _item) 500.0)
        ;;[1 1 1] Magic Happens Here
        (`PrimitiveComponent.SetRenderCustomDepth` _item false)))))

(event `self.ReceiveActorBeginOverlap`
  (params (OtherActor :type "Actor Object Reference"))
  (bind _item (`KismetArrayLibrary.Array_Get` (`self.K2_GetComponentsByClass` OtherActor "/Script/Engine.StaticMeshComponent")))
  ;[1 1 1] Movable Objects Glow
  (if (`KismetSystemLibrary.IsValid` _item)
    (if (`SceneComponent.IsAnySimulatingPhysics` _item)
      (if (< (`PrimitiveComponent.GetMass` _item) 500.0)
        (`KismetArrayLibrary.Array_Add` (`self.OverlappingTKActors`) OtherActor)))))

(event `self.ReceiveTick`
  (params (DeltaSeconds :type "Float (single-precision)"))
  (bind (_returnvalue_x _returnvalue_y) (`KismetMathLibrary.BreakVector2D` (`WidgetLayoutLibrary.GetViewportSize`)))
  (for _array_element (`self.OverlappingTKActors`)
    (bind _screenlocation (`PlayerController.ProjectWorldLocationToScreen` (`GameplayStatics.GetPlayerController` 0) (`self.K2_GetActorLocation` _array_element)))
    (if (and (> (`KismetMathLibrary.BreakVector2D` _screenlocation) 0.0) (> (`.Y` (`KismetMathLibrary.BreakVector2D` _screenlocation)) 0.0) (< (`KismetMathLibrary.BreakVector2D` _screenlocation) _returnvalue_x) (< (`.Y` (`KismetMathLibrary.BreakVector2D` _screenlocation)) _returnvalue_y))
      (bind _item (`KismetArrayLibrary.Array_Get` (`self.K2_GetComponentsByClass` _array_element "/Script/Engine.StaticMeshComponent")))
      ;[1 1 1] Magic Happens Here
      (`PrimitiveComponent.SetRenderCustomDepth` _item true)
      (`PrimitiveComponent.SetCustomDepthStencilValue` _item 255))))

(fn `UserConstructionScript`)