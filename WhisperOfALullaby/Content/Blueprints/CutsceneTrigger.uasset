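; A trigger actor that starts a numbered dialogue cutscene for the third-person character.
; On BeginPlay it creates a Cutscene widget in the viewport and starts it, passing its dialogue reference, if the character already overlaps the collision component.
; Unless OnlyOnLevelStart is set, a later overlap by the character also starts it, gated by a DoOnce that the BeginPlay path does not pass through.
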(event `self.ReceiveBeginPlay`
  (bind _returnvalue (`|CreateWidget` "/Game/2DNonDiegetic/Cutscenes/Cutscene.Cutscene_C" (`GameplayStatics.GetPlayerController` 0)))
  (bind _output_get (set `self.CutsceneWidget` _returnvalue))
  (`UserWidget.AddToViewport` _output_get 0)
  (`/Game/Blueprints/BlueprintDialogues/Utilities/Blueprints/Libs/Lib_Object_UtilityMacros.SafeGetArrayElement` (`PrimitiveComponent.GetOverlappingActors` (`self.CollisionComponent`) "/Game/Blueprints/Player/ThirdPersonCharacter.ThirdPersonCharacter_C")
    (:`then`
      (`/Game/2DNonDiegetic/Cutscenes/Cutscene.StartCutscene` (`self.CutsceneWidget`) (`self.CutsceneNum`) (`self.BPC_CutsceneDialogue`) false))))

(event `self.ReceiveActorBeginOverlap`
  (params (OtherActor :type "Actor Object Reference"))
  (if (not (`self.OnlyOnLevelStart`))
    (cast `/Game/Blueprints/Player/ThirdPersonCharacter` OtherActor)
    (`/Engine/EditorBlueprintResources/StandardMacros.DoOnce` false
      (:`Completed`
        (`/Game/2DNonDiegetic/Cutscenes/Cutscene.StartCutscene` (`self.CutsceneWidget`) (`self.CutsceneNum`) (`self.BPC_CutsceneDialogue`) false)))))

(fn `UserConstructionScript`)