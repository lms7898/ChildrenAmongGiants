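; LeverManager tracks a set of required levers and flags when all of them have been pulled.
; On BeginPlay it binds LeverPull to the lever interaction event.
; Each call recounts the pulled entries in RequiredLevers and sets AllPulled when the count matches the array length.
; Nothing here clears AllPulled once it is set, and Tick is unused.
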(event `self.ReceiveBeginPlay`
  (add `self.LeverInteraction` (delegate `LeverPull`)))

(event `LeverPull`
  (bind _output_get (set `self.LeverCounter` 0))
  (for _array_element (`self.RequiredLevers`)
    (if (`/Game/Blueprints/Lever.Pulled` _array_element)
      (bind _result (`/Game/BlueprintDialogues/Utilities/Blueprints/Libs/Lib_Math.Increment (int)` _output_get 1))
      (set `self.LeverCounter` _result)))
  (if (== (`self.LeverCounter`) (`KismetArrayLibrary.Array_Length` (`self.RequiredLevers`)))
    (set `self.AllPulled` true)
    (else
      (set `self.LeverCounter` 0))))