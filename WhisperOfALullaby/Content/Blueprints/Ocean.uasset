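; Ocean actor that slides back and forth along X like a tide and carries overlapping Pawns with it.
; Each Tick sets its X from a game-time sine wave, offset behind its start position, and stores the change since last frame.
; Overlapping Pawns get a swept location offset combining a constant negative-X current with that wave change, plus a smaller vertical bob.
; An older velocity-based push remains but is disconnected.
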(event `self.ReceiveBeginPlay`
  (bind _output_get (set `self.StartLocation` (`self.K2_GetActorLocation`)))
  (set `self.StartX` (.x _output_get)))

(event `self.ReceiveTick`
  (params (DeltaSeconds :type "Float (single-precision)"))
  (bind (_returnvalue_x _returnvalue_y _returnvalue_z) (`KismetMathLibrary.BreakVector` (`self.K2_GetActorLocation`)))
  (bind _wavedelta (`self.WaveDelta`))
  (bind _returnvalue (* (`self.WaveDist`) (`KismetMathLibrary.Sin` (* (`KismetSystemLibrary.GetGameTimeInSeconds`) 0.5))))
  (set `self.dt` DeltaSeconds)
  (set `self.WaveDelta` (- _returnvalue (`self.WavePrevExtent`)))
  (set `self.WavePrevExtent` _returnvalue)
  ;[1 1 1] Move the ocean in and out on a Sin wave
  (`self.K2_SetActorLocation` (`KismetMathLibrary.MakeVector` (- (+ _returnvalue (`self.StartX`)) (`self.WaveDist`)) _returnvalue_y _returnvalue_z))
  ;[1 1 1] Push Objects In the Ocean
  (for _array_element (`self.GetOverlappingActors` null)
    (bind _aspawn (cast `Pawn` _array_element))
    (set `self.PerFrameOffset` (`KismetMathLibrary.MakeVector` (+ (* (`self.dt`) -400.0) (* _wavedelta 1.0)) 0.0 (* _wavedelta 0.3)))
    (`self.K2_SetActorLocation` _aspawn (+ (`self.K2_GetActorLocation` _aspawn) (`self.PerFrameOffset`)) true false)))

(fn `UserConstructionScript`)