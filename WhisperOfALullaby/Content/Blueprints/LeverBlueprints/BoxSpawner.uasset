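; BoxSpawner is a lever-driven actor that repositions a set of existing boxes rather than spawning new ones.
; On BeginPlay it binds its Interaction event to LeverManager1's lever interaction.
; Each interaction teleports every entry in Boxes to a base position plus its own offset, with zero rotation.
; Offsets come from the flat OffsetXYZ array, read as consecutive X, Y, Z triples by box index.
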(event `self.ReceiveBeginPlay`
  (add `/Game/Blueprints/LeverBlueprints/LeverManager.LeverInteraction` (`self.LeverManager1`) (delegate `Interaction`)))

(event `Interaction`
  (bind _offsetxyz (`self.OffsetXYZ`))
  (for (_array_element _array_index) (`self.Boxes`)
    (bind _returnvalue (* _array_index 3))
    (`self.K2_TeleportTo` :`self` _array_element :`DestLocation` (`KismetMathLibrary.MakeVector` (+ (`self.PositionX`) (`KismetArrayLibrary.Array_Get` _offsetxyz (+ _returnvalue 0))) (+ (`self.PositionY`) (`KismetArrayLibrary.Array_Get` _offsetxyz (+ _returnvalue 1))) (+ (`self.PositionZ`) (`KismetArrayLibrary.Array_Get` _offsetxyz (+ _returnvalue 2)))))))

(fn `UserConstructionScript`)