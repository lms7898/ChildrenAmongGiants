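; KeyManager is a Blueprint that tracks whether a level's door is open and announces the level clear.
; The OpenSesame event sets Open to true and prints the success message.
; A check that counts collected entries in RequiredKeys, then opens or prints "Locked!", is unconnected to any event and never runs.
; OpenSesame therefore opens without verifying keys.
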(event `OpenSesame`
  (set `self.Open` true)
  (`KismetSystemLibrary.PrintText` "The Door Is Open! Level Clear!" true true (struct :`R` 1.0 :`G` 0.09546 :`B` 0.038127 :`A` 1.0)))