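; Elliana is an actor Blueprint that moves itself along a straight line between Start and End.
; While LERPing is set, Tick lerps its location using milliseconds of StartTime minus Now, divided by Duration, as alpha.
; AdvanceTarget steps through TargetPoints into CurrentTarget, which the movement does not read.
; Nothing in this graph sets the lerp variables or flag.
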(event `AdvanceTarget`
  ;[1 1 1] Advance target point
  (set `self.PointsIndex` (+ (`self.PointsIndex`) 1))
  (set `self.currentTarget` (`KismetArrayLibrary.Array_Get` (`self.TargetPoints`) (`self.PointsIndex`))))

(event `self.ReceiveTick`
  (params (DeltaSeconds :type "Float (single-precision)"))
  (if (`self.LERPing`)
    (`self.K2_SetActorLocation` (`KismetMathLibrary.VLerp` (`self.start`) (`self.end`) (/ (`KismetMathLibrary.GetTotalMilliseconds` (- (`self.startTime`) (`KismetMathLibrary.Now`))) (`self.duration`))))))

(fn `UserConstructionScript`)