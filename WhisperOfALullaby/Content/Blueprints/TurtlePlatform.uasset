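; TurtlePlatform is an AI-driven moving platform that walks back and forth between two bound actors, LBound and RBound.
; BeginPlay caches its AI controller and starts in Idle, from which the first move heads right.
; Tick polls the controller's move status, and each time it goes idle a DoOnce flips the walking state and issues SimpleMoveToActor toward the other bound.
; The DoOnce re-arms while the platform is moving.
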(event `self.ReceiveBeginPlay`
  ;[1 1 1] Initialize
  ;;[1 1 1] Start Idle
  (set `self.state` "NewEnumerator0")
  ;;[1 1 1] Get AiController ref
  (bind _returnvalue (`AIBlueprintHelperLibrary.GetAIController` self))
  (set `self.ai` _returnvalue))

(event `self.ReceiveTick`
  (params (DeltaSeconds :type "Float (single-precision)"))
  ;[1 1 1] Walk Back And Forth
  (switch `EPathFollowingStatus` (`AIController.GetMoveStatus` (`self.ai`))
    (:`Idle`
      (`/Engine/EditorBlueprintResources/StandardMacros.DoOnce` false :!label _label
        (:`Completed`
          (switch `/Game/Blueprints/PacingCharacterState` (`self.state`)
            (:`NewEnumerator0`
              (set `self.state` "NewEnumerator2")
              (`NavigationSystem.SimpleMoveToActor` (`self.ai`) (`self.r_bound`)))
            (:`NewEnumerator1`
              (`NavigationSystem.SimpleMoveToActor` (`self.ai`) (`self.r_bound`))
              (set `self.state` "NewEnumerator2"))
            (:`NewEnumerator2`
              (`NavigationSystem.SimpleMoveToActor` (`self.ai`) (`self.l_bound`))
              (set `self.state` "NewEnumerator1"))))))
    (:`Moving`
      (goto _label :!via `Reset`))))

(fn `UserConstructionScript`)