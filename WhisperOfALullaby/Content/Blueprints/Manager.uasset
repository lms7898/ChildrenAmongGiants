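; Level manager that switches the scene's mood when the player jumps or falls.
; It caches the player, dolls, skylight and two ambient sounds on begin play, relying on array order, and grabs crowd actors once spawned.
; Jumping triggers every doll's chase and swaps crowd noise for heartbeat; falling restores crowd noise.
; Both events set the skylight visible; teleport logic for moving player and dolls is unused.
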(event `self.ReceiveBeginPlay`
  ;[1 1 1] Get Player
  (bind _outactors (`GameplayStatics.GetAllActorsOfClass` null))
  (set `self.playerRef` (`KismetArrayLibrary.Array_Get` _outactors))
  ;[1 1 1] Get Dolls
  (bind _outactors_2 (`GameplayStatics.GetAllActorsOfClass` "/Game/Blueprints/Doll.Doll_C"))
  (set `self.dolls` _outactors_2)
  ;[1 1 1] Get Light Reference
  (bind _outactors_3 (`GameplayStatics.GetAllActorsOfClass` "/Script/Engine.SkyLight"))
  (set `self.light` (`KismetArrayLibrary.Array_Get` _outactors_3))
  ;[1 1 1] Get Ambient
  (bind _outactors_4 (`GameplayStatics.GetAllActorsOfClass` "/Script/Engine.AmbientSound"))
  (set `self.crowdNoise` (`KismetArrayLibrary.Array_Get` _outactors_4))
  (set `self.Heartbeat` (`KismetArrayLibrary.Array_Get` _outactors_4 1)))

(event `CrowdSpawned`
  ;[1 1 1] Get Crowd Memebers
  (bind _outactors (`GameplayStatics.GetAllActorsOfClass` "/Game/Blueprints/CrowdSpawner_Blueprint.CrowdSpawner_Blueprint_C"))
  (set `self.crowdMemebers` (`/Game/Blueprints/CrowdSpawner_Blueprint.crowdActors` (`KismetArrayLibrary.Array_Get` _outactors))))

(event `PlayerJumps`
  (for _array_element (`self.dolls`)
    ;[1 1 1] Activate Doll Chase
    (bind _asdoll (cast `/Game/Blueprints/Doll` _array_element))
    (`/Game/Blueprints/Doll.PlayerJumped` _asdoll)
    ;[1 1 1] Hit the Lights
    (`SceneComponent.SetVisibility` (`SkyLight.LightComponent` (`self.light`)) true false)
    ;[1 1 1] Sound On/Off
    (`AudioComponent.SetVolumeMultiplier` (`AmbientSound.AudioComponent` (`self.crowdNoise`)) 0.0) ; mute crowd
    (`AudioComponent.SetVolumeMultiplier` (`AmbientSound.AudioComponent` (`self.Heartbeat`)) 5.0) ; play heartbeat
  ))

(event `PlayerFalls`
  ;[1 1 1] Hit the Lights
  (`SceneComponent.SetVisibility` (`SkyLight.LightComponent` (`self.light`)) true false)
  ;[1 1 1] Sound On/Off
  (`AudioComponent.SetVolumeMultiplier` (`AmbientSound.AudioComponent` (`self.crowdNoise`)) 0.1) ; play crowd
  (`AudioComponent.SetVolumeMultiplier` (`AmbientSound.AudioComponent` (`self.Heartbeat`)) 0.0) ; play crowd
)

(fn `UserConstructionScript`)