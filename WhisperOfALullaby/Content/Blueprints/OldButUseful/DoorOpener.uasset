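; DoorOpener is a Blueprint that opens a door once four colored keys (Cyan, Green, Orange and Purple) are all found.
; Each color has its own event that sets a done flag and feeds a shared check of all four flags.
; When all flags are true it plays the Door matinee, otherwise it prints a debug message that keys are missing.
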(event `Cyan`
  (set `self.CyanDone` true)
  (if (and (and (`self.CyanDone`) (`self.GreenDone`)) (and (`self.OrangeDone`) (`self.PurpleDone`))) :!label _label
    (`MatineeActor.Play` (`self.Door`))
    (`KismetSystemLibrary.PrintText` "matinee play")
    (else
      (`KismetSystemLibrary.PrintText` "not all keys found"))))

(event `Green`
  (set `self.GreenDone` true)
  (goto _label))

(event `Orange`
  (set `self.OrangeDone` true)
  (goto _label))

(event `Purple`
  (set `self.PurpleDone` true)
  (goto _label))

(fn `UserConstructionScript`)