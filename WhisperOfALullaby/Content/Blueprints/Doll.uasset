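; Doll is an enemy that chases the player for a limited time and turns into a crowd after ten seconds.
; Seeing a pawn through PawnSensing issues a move toward it, while PlayerJumped refills a chase timer.
; Tick counts that timer down, re-issuing SimpleMoveToActor toward the player while it remains positive.
; A BeginPlay timer spawns CrowdBP at the doll's transform and destroys the doll.
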(event `self.PawnSensing.OnSeePawn`
  (params (Pawn :type "Pawn Object Reference"))
  ;[1 1 1] Simple Chase Player (from clown BP)
  (`NavigationSystem.SimpleMoveToActor` (`self.GetController`) Pawn))

(event `PlayerJumped`
  ;[1 1 1] begin chase if spotted
  (set `self.chaseTimer` (`self.maxChaseTimer`)))

(event `self.ReceiveTick`
  (params (DeltaSeconds :type "Float (single-precision)"))
  (set `self.chaseTimer` (- (`self.chaseTimer`) DeltaSeconds))
  ;[1 1 1] Chase player
  (if (> (`self.chaseTimer`) 0.0)
    (bind _returnvalue (`AIBlueprintHelperLibrary.GetAIController` (`self.GetController`)))
    (`NavigationSystem.SimpleMoveToActor` (`self.GetController`) (`GameplayStatics.GetPlayerPawn` 0))
    (else
      (set `self.pursuing` false))))

(event `self.ReceiveBeginPlay`
  (`KismetSystemLibrary.K2_SetTimerDelegate` (delegate `ReplaceWithCrowd`) 10.0))

(event `ReplaceWithCrowd`
  (`|SpawnActorFromClass` "/Game/Blueprints/CrowdBP.CrowdBP_C" (`self.GetTransform`) "AlwaysSpawn" "OverrideRootScale")
  (`self.K2_DestroyActor`))

(fn `UserConstructionScript`)