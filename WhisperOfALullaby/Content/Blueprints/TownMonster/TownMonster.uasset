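; Town monster character that wanders between random TargetPoints until it overlaps a Malice Sphere, then chases the player.
; Tick runs a two-state Mode: wandering picks a new waypoint when movement stops and teleports the monster if stuck too long; chasing hits the player whenever AI movement is idle.
; Overlapping the player character also applies damage, and falling below zero height destroys the monster.
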(event `self.ReceiveBeginPlay`
  (bind _targetpoints (`self.TargetPoints`))
  ;[1 1 1] On Start
  ;;[1 1 1] Get The List of Waypoints
  (bind _outactors (`GameplayStatics.GetAllActorsOfClass` "/Script/Engine.TargetPoint"))
  (bind _output_get (set `self.TargetPoints` _outactors))
  (set `self.CurrentTarget` (`KismetArrayLibrary.Array_Get` _output_get))
  (set `self.lastMovement` (`KismetSystemLibrary.GetGameTimeInSeconds`))
  ;;[1 1 1] Get First Target Point
  (set `self.currentTarget` (`KismetArrayLibrary.Array_Get` _targetpoints (`KismetMathLibrary.RandomInteger` (`KismetArrayLibrary.Array_Length` _targetpoints))))
  ;;[1 1 1] Set AI Controller Reference
  (bind _returnvalue (`AIBlueprintHelperLibrary.GetAIController` self))
  (set `self.AI` _returnvalue))

(event `self.ReceiveActorBeginOverlap`
  (params (OtherActor :type "Actor Object Reference"))
  ;[1 1 1] Handle Collisions And Player Detection
  ;;[1 1 1] Overlap
  (switch `string` (`KismetSystemLibrary.GetClassDisplayName` (`GameplayStatics.GetObjectClass` OtherActor))
    (:`MaliceSphere_C`
      ;;[1 1 1] Chase Player
      (`self.ChasePlayer`))
    (:`ThirdPersonCharacter_C`
      ;;[1 1 1] Damage
      (`GameplayStatics.ApplyDamage` OtherActor 19.0 null self))))

(event `self.ReceiveTick`
  (params (DeltaSeconds :type "Float (single-precision)"))
  ;[1 1 1] Move Randomly
  ;;[1 1 1] Tick
  ;;[1 1 1] Out of bounds
  (if (< (.z (.location (`self.GetTransform`))) 0.0)
    (`self.K2_DestroyActor`)
    (else
      ;;[1 1 1] Movement Mode
      (switch `int` (`self.mode`) ; (0) wandering (1) chasing
        (:`0`
          ;;[1 1 1] If Character is not moving
          (if (< (`KismetMathLibrary.VSize` (`MovementComponent.Velocity` (`self.CharacterMovement`))) 1.0)
            ;;[1 1 1] If Stuck, Set New Waypoint
            (`self.SetRandomWaypoint`)
            ;;[1 1 1] Check Permanently Stuck
            (if (> (- (`KismetSystemLibrary.GetGameTimeInSeconds`) (`self.lastMovement`)) 1.0)
              ;;[1 1 1] Reset
              (`self.Reset`)
              (else
                ;;[1 1 1] Walk
                (`NavigationSystem.SimpleMoveToActor` (`self.GetController`) (`self.currentTarget`))
                (set `self.lastMovement` (`KismetSystemLibrary.GetGameTimeInSeconds`))))
            (else
              ;;[1 1 1] Moved
              (set `self.lastMovement` (`KismetSystemLibrary.GetGameTimeInSeconds`)))))
        (:`1`
          ;;[1 1 1] When target found
          (switch `EPathFollowingStatus` (`AIController.GetMoveStatus` (`self.AI`))
            (:`Idle`
              ;;[1 1 1] Damage
              (bind _asthird_person_character (cast `/Game/Blueprints/ThirdPersonCharacter` (`GameplayStatics.GetPlayerPawn` 0)))
              (`/Game/Blueprints/ThirdPersonCharacter.Hit` _asthird_person_character 20.0)
              (`KismetSystemLibrary.PrintString` "Hello"))))))))

(fn `ChasePlayer`
  ;[1 1 1] Chase player
  (`AIBlueprintHelperLibrary.GetAIController` (`self.GetController`))
  (`NavigationSystem.SimpleMoveToActor` (`self.GetController`) (`GameplayStatics.GetPlayerPawn` 0))
  (set `self.mode` 1))

(fn `Reset`
  ;[1 1 1] If permanently stuck, reset
  (`self.K2_SetActorLocation` (`KismetMathLibrary.MakeVector` 700.0 (+ (* (`KismetMathLibrary.RandomFloat`) -1000.0) -7000.0) 3770.0) false true)
  (set `self.MovementLocked` false)
  (set `self.lastMovement` (`KismetSystemLibrary.GetGameTimeInSeconds`))
  (return))

(fn `SetRandomWaypoint`
  (bind _targetpoints (`self.TargetPoints`))
  ;[1 1 1] Set New Target Point
  (set `self.currentTarget` (`KismetArrayLibrary.Array_Get` _targetpoints (`KismetMathLibrary.RandomInteger` (`KismetArrayLibrary.Array_Length` _targetpoints)))))

(fn `UserConstructionScript`)