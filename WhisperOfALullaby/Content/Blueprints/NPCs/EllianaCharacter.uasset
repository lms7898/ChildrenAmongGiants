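; EllianaCharacter is an NPC that travels a scripted route through an indexed list of KeyPoints actors.
; AdvanceTarget steps the index and switches per point between AI navmesh movement and straight-line teleporting lerps, setting whether arrival auto-advances or stops.
; Tick drives whichever mode is active, timing lerps by distance over LERPspeed and ending navmesh moves within a proximity threshold.
; GoToTargetPointNum sends the character by navmesh to any chosen point.
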(event `self.ReceiveBeginPlay`
  ;[1 1 1] Start
  (bind _returnvalue (`AIBlueprintHelperLibrary.GetAIController` self))
  (set `self.AI` _returnvalue))

(event `AdvanceTarget`
  ;[1 1 1] Advance target point (navmesh)
  (set `self.PointsIndex` (+ (`self.PointsIndex`) 1))
  (`self.UpdateGoal`)
  (switch `int` (`self.pointsIndex`)
    (:`1`
      (`self.AdvanceTarget`))
    (:`2`
      (set `self.AutoAdvance` false)
      (set `self.UseNavMesh` true :!label _label))
    (:`3`
      (set `self.AutoAdvance` true :!label _label_2)
      (`self.LERPToLocation` (`self.CurrentTarget`) :!label _label_3))
    (:`4`
      (set `self.AutoAdvance` true :!label _label_4)
      (goto _label))
    (:`5`
      (set `self.AutoAdvance` false :!label _label_5)
      (goto _label_3))
    (:`6`
      (goto _label_2))
    (:`7`
      (goto _label_4))
    (:`8`
      (goto _label_5))))

(event `self.ReceiveTick`
  (params (DeltaSeconds :type "Float (single-precision)"))
  (bind _currenttarget (`self.CurrentTarget`))
  (bind _returnvalue (/ (`KismetMathLibrary.GetTotalMilliseconds` (- (`KismetMathLibrary.Now`) (`self.startTime`))) (`self.duration`)))
  ;[1 1 1] Tick
  (if (`self.LERPing`)
    ;[1 1 1] LERP
    (`self.K2_SetActorLocation` (`KismetMathLibrary.VLerp` (`self.start`) (`self.end`) _returnvalue) false true)
    (if (> _returnvalue 1.0)
      (set `self.LERPing` false)
      (if (`self.AutoAdvance`)
        (`self.AdvanceTarget`)))
    (else
      ;[1 1 1] Use Nav Mesh To Point
      (if (`self.UseNavMesh`)
        (`NavigationSystem.SimpleMoveToLocation` (`self.AI`) _currenttarget)
        (if (< (`KismetMathLibrary.VSizeSquared` (- _currenttarget (`self.K2_GetActorLocation`))) 10000.0)
          (set `self.UseNavMesh` false)
          (if (`self.AutoAdvance`)
            (`self.AdvanceTarget`)))))))

(event `LERPToLocation`
  (params (NewLocation :type "Vector Structure"))
  ;[1 1 1] Set LERP Target
  (set `self.end` NewLocation)
  (set `self.start` (`self.K2_GetActorLocation`))
  (set `self.startTime` (`KismetMathLibrary.Now`))
  (set `self.LERPing` true)
  (set `self.duration` (/ (`KismetMathLibrary.VSize` (- (`self.end`) (`self.start`))) (`self.LERPspeed`))))

(event `GoToTargetPointNum`
  (params (num :type Integer))
  ;[1 1 1] Nav to Point
  (set `self.PointsIndex` num)
  (set `self.CurrentTarget` (`self.K2_GetActorLocation` (`KismetArrayLibrary.Array_Get` (`self.KeyPoints`) (`self.pointsIndex`))))
  (set `self.UseNavMesh` true))

(fn `UserConstructionScript`)