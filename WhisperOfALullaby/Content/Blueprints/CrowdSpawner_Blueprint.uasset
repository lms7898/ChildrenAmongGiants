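; CrowdSpawner is an actor Blueprint that populates the level with crowd actors when play begins.
; It spawns CrowdBP instances in a loop driven by CrowdSize, at random horizontal positions within a fixed rectangle and at a constant height, adjusting for collisions but always spawning.
; Each instance is stored in CrowdActors, then the first Manager found in the level is notified through CrowdSpawned.
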(event `self.ReceiveBeginPlay`
  (for _ (range (+ (`self.CrowdSize`) 1))
    (bind _returnvalue (`|SpawnActorFromClass` "/Game/Blueprints/CrowdBP.CrowdBP_C" (`KismetMathLibrary.Conv_VectorToTransform` (`KismetMathLibrary.MakeVector` (`KismetMathLibrary.RandomFloatInRange` -4000.0 4000.0) (`KismetMathLibrary.RandomFloatInRange` -1200.0 1200.0) 100.0)) "AdjustIfPossibleButAlwaysSpawn" "OverrideRootScale")) ; Spawn Crowd
    (`KismetArrayLibrary.Array_Add` (`self.crowdActors`) _returnvalue))
  (bind _outactors (`GameplayStatics.GetAllActorsOfClass` "/Game/Blueprints/Manager.Manager_C"))
  (bind _asmanager (cast `/Game/Blueprints/Manager` (`KismetArrayLibrary.Array_Get` _outactors)))
  (`/Game/Blueprints/Manager.CrowdSpawned` _asmanager))

(fn `UserConstructionScript`)