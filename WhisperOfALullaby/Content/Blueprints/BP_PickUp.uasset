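; Pickup actor that spins and bobs in place until the player character touches it.
; Tick rotates the static mesh a fixed step per frame and plays the FloatUpDown timeline, whose curve value is added as a local offset on each update.
; An overlap with an actor of exactly the ThirdPersonCharacter class sets the Collected flag and hides the actor rather than destroying it.
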(event `self.ReceiveTick`
  (params (DeltaSeconds :type "Float (single-precision)"))
  (`SceneComponent.K2_AddLocalRotation` (`self.StaticMesh`) (struct :`Yaw` 1.0) false false)
  (bind (_direction _updown) (`Timeline|FloatUpDown`)
    (:`Update`
      (`SceneComponent.K2_AddLocalOffset` (`self.StaticMesh`) _updown false false))))

(event `self.ReceiveActorBeginOverlap`
  (params (OtherActor :type "Actor Object Reference"))
  (if (== (`GameplayStatics.GetObjectClass` OtherActor) "/Game/Blueprints/ThirdPersonCharacter.ThirdPersonCharacter_C")
    (set `self.Collected` true)
    (`self.SetActorHiddenInGame` true)))

(fn `UserConstructionScript`)