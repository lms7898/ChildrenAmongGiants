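; KeyManagerTemp is a temporary-named key manager that gates a level-ending door on collected keys.
; OpenSesame loops over RequiredKeys, checking each Collected flag, then compares KeyCounter to the array length to set Open and print a level-clear or locked message.
; As wired, KeyCounter resets to zero right after each increment, so the check passes only when RequiredKeys is empty.
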(event `OpenSesame`
  (bind _output_get (set `self.KeyCounter` 0))
  (for _array_element (`self.RequiredKeys`)
    (if (`/Game/Blueprints/BP_PickUp.Collected` _array_element)
      (`/Game/BlueprintDialogues/Utilities/Blueprints/Libs/Lib_Math.Increment (int)` _output_get 1)
      (set `self.KeyCounter` 0)))
  (if (== (`self.KeyCounter`) (`KismetArrayLibrary.Array_Length` (`self.RequiredKeys`)))
    (set `self.Open` true)
    (`KismetSystemLibrary.PrintText` "The Door Is Open! Level Clear!" true true (struct :`R` 1.0 :`G` 0.09546 :`B` 0.038127 :`A` 1.0))
    (else
      (set `self.KeyCounter` 0)
      (`KismetSystemLibrary.PrintText` "Locked!" true true (struct :`R` 1.0 :`G` 0.164194 :`B` 0.097282 :`A` 1.0)))))