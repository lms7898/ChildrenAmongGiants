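; InputListener is an actor that waits for any key press, records the player's input type and opens the MainMenu level.
; Three Any Key handlers classify the pressed key as keyboard, mouse button or gamepad.
; Each writes an InputType enum to MyGameInstance before the level change, with keyboard and mouse sharing one value and gamepad using another.
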(event `Key|AnyKey`
  (params (Key :type "Key Structure" :default "AnyKey"))
  ;[1 1 1] Determine Input Type Based on Key Pressed
  (:`Pressed`
    (if (`KismetInputLibrary.Key_IsKeyboardKey` Key)
      (bind _asmy_game_instance (cast `/Game/GameInstances/MyGameInstance` (`GameplayStatics.GetGameInstance`)))
      (set `/Game/GameInstances/MyGameInstance.InputType` "NewEnumerator0" _asmy_game_instance)
      (`GameplayStatics.OpenLevel` "MainMenu"))))

(event `Key|AnyKey`
  (params (Key :type "Key Structure" :default "AnyKey"))
  ;[1 1 1] Determine Input Type Based on Key Pressed
  (:`Pressed`
    (if (`KismetInputLibrary.Key_IsMouseButton` Key)
      (bind _asmy_game_instance (cast `/Game/GameInstances/MyGameInstance` (`GameplayStatics.GetGameInstance`)))
      (set `/Game/GameInstances/MyGameInstance.InputType` "NewEnumerator0" _asmy_game_instance)
      (`GameplayStatics.OpenLevel` "MainMenu"))))

(event `Key|AnyKey`
  (params (Key :type "Key Structure" :default "AnyKey"))
  ;[1 1 1] Determine Input Type Based on Key Pressed
  (:`Pressed`
    (if (`KismetInputLibrary.Key_IsGamepadKey` Key)
      (bind _asmy_game_instance (cast `/Game/GameInstances/MyGameInstance` (`GameplayStatics.GetGameInstance`)))
      (set `/Game/GameInstances/MyGameInstance.InputType` "NewEnumerator1" _asmy_game_instance)
      (`GameplayStatics.OpenLevel` "MainMenu"))))

(fn `UserConstructionScript`)