(event `/Game/BlueprintDialogues/UseSystem/Blueprints/Interfaces/BPI_Usable.Use`
  (params (PC :type "PlayerController Object Reference"))
  (`KismetSystemLibrary.PrintString` "You used me!!!!!!" true true (struct :`R` 0.755 :`B` 0.546502 :`A` 1.0)))