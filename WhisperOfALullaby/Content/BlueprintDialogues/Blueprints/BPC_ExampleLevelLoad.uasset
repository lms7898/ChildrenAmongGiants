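; Example dialogue Blueprint that supplies level-load dialogue from the DT_Dialogue_LevelLoad data table.
; On Tick it reads the game instance's input type, setting the matching input type and initial branch for mouse/keyboard or Xbox 360.
; Overridable functions serve row names and items, with item lookup switched on the current level name.
; The script interpreter comes from ThirdPersonGameMode.
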(event `self.ReceiveTick`
  (params (DeltaSeconds :type "Float (single-precision)"))
  (bind _asmy_game_instance (cast `/Game/GameInstances/MyGameInstance` (`GameplayStatics.GetGameInstance`)))
  (switch `/Game/GameInstances/InputType` (`/Game/GameInstances/MyGameInstance.InputType` _asmy_game_instance)
    (:`NewEnumerator0`
      (`self.SetInputType` "NewEnumerator0")
      (set `self.InitialBranch` "aMK_1"))
    (:`NewEnumerator1`
      (`self.SetInputType` "NewEnumerator1")
      (set `self.InitialBranch` "aXB360_1"))))

(fn `GetDialogueItem`
  (params (ItemName :type Name))
  (returns (Item :type "/Game/BlueprintDialogues/Blueprints/Structures/Dialogue_TableItem Structure") (Found :type Boolean))
  ;[1 0 1] Override this function for derived classes using another data table
  (bind _returnvalue (`GameplayStatics.GetCurrentLevelName` true))
  (switch `string` _returnvalue
    (:`ThirdPersonExampleMap`
      (bind _returnvalue_2 (`|GetDataTableRow` "/Game/BlueprintDialogues/Data/DT_Dialogue_LevelLoad.DT_Dialogue_LevelLoad" ItemName)
        (:`then`
          (bind _result (`/Game/BlueprintDialogues/Utilities/Blueprints/Libs/Lib_Object_UtilityMacros.MakeBoolFromBranch` :!label _label))
          (return _returnvalue_2 _result))
        (:`RowNotFound`
          (goto _label :!via `False`))))))

(fn `GetDialogueRowNames`
  (returns (Names :type "Array of Name"))
  ;[1 0 1] Override this function for derived classes using another data table
  (bind _returnvalue (`GameplayStatics.GetCurrentLevelName` true))
  (switch `string` _returnvalue
    (:`Default`
      _)
    (:`ThirdPersonExampleMap`
      _))
  (bind _outrownames (`DataTableFunctionLibrary.GetDataTableRowNames` "/Game/BlueprintDialogues/Data/DT_Dialogue_LevelLoad.DT_Dialogue_LevelLoad"))
  (return _outrownames))

(fn `GetScriptInterpreter`
  (returns (Interpreter :type "/Game/BlueprintDialogues/ScriptSystem/Blueprints/BP_ScriptInterpreter Object Reference"))
  (return (`/Game/GameModes/ThirdPersonGameMode.SciptInterp` (cast `/Game/GameModes/ThirdPersonGameMode` (`GameplayStatics.GetGameMode`) :!pure true))))