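; BPC_ExampleDialogue is an example dialogue component that fetches rows from DT_Dialogue_Example and exposes the game mode's script interpreter.
; GetDialogueItem picks a hardcoded row by the game instance's input type, keyboard or Xbox 360, ignoring its ItemName argument.
; It prints debug text and returns a found flag, but its Item output is wired only to the Xbox lookup.
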(fn `GetDialogueItem`
  (params (ItemName :type Name))
  (returns (Item :type "/Game/BlueprintDialogues/Blueprints/Structures/Dialogue_TableItem Structure") (Found :type Boolean))
  (bind _asmy_game_instance (cast `/Game/GameInstances/MyGameInstance` (`GameplayStatics.GetGameInstance`)))
  (bind _inputtype (`/Game/GameInstances/MyGameInstance.InputType` _asmy_game_instance))
  (switch `/Game/GameInstances/InputType` _inputtype
    (:`NewEnumerator0`
      (`|GetDataTableRow` "/Game/BlueprintDialogues/Data/DT_Dialogue_Example.DT_Dialogue_Example" "KM1"
        (:`then`
          (`KismetSystemLibrary.PrintText` "Row Found" :!label _label))
        (:`RowNotFound`
          (`KismetSystemLibrary.PrintText` "Row Not Found" :!label _label_2))))
    (:`NewEnumerator1`
      (bind _returnvalue (`|GetDataTableRow` "/Game/BlueprintDialogues/Data/DT_Dialogue_Example.DT_Dialogue_Example" "XB3601")
        (:`then`
          (goto _label))
        (:`RowNotFound`
          (goto _label_2)))))
  (`KismetSystemLibrary.PrintText` (`KismetTextLibrary.Conv_StringToText` (`KismetStringLibrary.Conv_ByteToString` _inputtype)) true true (struct :`R` 1.0 :`G` 0.118581 :`B` 0.166353 :`A` 1.0))
  (bind _result (`/Game/BlueprintDialogues/Utilities/Blueprints/Libs/Lib_Object_UtilityMacros.MakeBoolFromBranch`))
  (return _returnvalue _result))

(fn `GetScriptInterpreter`
  (returns (Interpreter :type "/Game/BlueprintDialogues/ScriptSystem/Blueprints/BP_ScriptInterpreter Object Reference"))
  (return (`/Game/Blueprints/ThirdPersonGameMode.SciptInterp` (cast `/Game/Blueprints/ThirdPersonGameMode` (`GameplayStatics.GetGameMode`) :!pure true))))